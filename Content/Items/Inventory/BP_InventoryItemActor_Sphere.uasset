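; BP_InventoryItemActor_Sphere is an inventory item actor that represents a sphere item.
; Its construction script runs the parent's, then copies the sphere's row from DT_GameItemDataTable into GameItem and sets InventoryMeta with a hardcoded item count and stack size.
; A missing row only prints an error, whose text mistakenly names the Cube actor.
; The event graph adds no logic of its own, with BeginPlay deferring to the parent.
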(event EventBeginPlay
  (|CallParentFunction))

(event Collision|EventActorBeginOverlap
  (params (OtherActor :type Actor%20Object%20Reference))
  (|CallParentFunction OtherActor) ; This node is disabled and will not be called.\nDrag off pins to build functionality.
)

(event EventTick
  (params (DeltaSeconds :type Float%20%28single-precision%29))
  (|CallParentFunction DeltaSeconds) ; This node is disabled and will not be called.\nDrag off pins to build functionality.
)

(fn ConstructionScript
  (|CallParentFunction)
  (bind _returnvalue (Utilities|GetDataTableRow "/Game/DataTable/DT_GameItemDataTable.DT_GameItemDataTable" "Item_Sphere_01")
    (:then
      (Variables|Default|SetGameItem _returnvalue)
      (Variables|Default|SetInventoryMeta (Utilities|Struct|MakeInventoryMetaStructure 3 5)))
    (:RowNotFound
      (Development|PrintString "Error: Cant fillup InventoryItemActorCube" true true "(R=1.000000,G=0.000000,B=0.044384,A=1.000000)"))))