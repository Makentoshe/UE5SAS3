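; Environment item actor that offers itself as a nearby interaction to actors holding an interactor component.
; On BeginPlay it binds overlap begin and end events, which add or remove its action on that component through BPI_ActorComponentInteractor_Holder.
; The action comes from GetNearbyActionStructure, whose Environment-type structure built from item title and description is left unused.
; The environment interaction event itself is empty.
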(event Custom|OnEnvironmentNearbyInteractionEvent)

(event Custom|OnNearbyInteractionBeginEvent
  (params (OverlappedActor :type Actor%20Object%20Reference))
  (if (Utilities|DoesObjectImplementInterface OverlappedActor "/Game/Features/Feature_Interaction/Interfaces/BPI_ActorComponentInteractor_Holder.BPI_ActorComponentInteractor_Holder_C")
    (bind _component (Class|BPIActorComponentInteractorHolder|GetInteractorActorComponent(Message) OverlappedActor))
    (Default|OnAddNearbyActionEvent _component (Utilities|GetNearbyActionStructure))))

(event Custom|OnNearbyInteractionEndEvent
  (params (OverlappedActor :type Actor%20Object%20Reference))
  (if (Utilities|DoesObjectImplementInterface OverlappedActor "/Game/Features/Feature_Interaction/Interfaces/BPI_ActorComponentInteractor_Holder.BPI_ActorComponentInteractor_Holder_C")
    (bind _component (Class|BPIActorComponentInteractorHolder|GetInteractorActorComponent(Message) OverlappedActor))
    (Default|OnRemoveNearbyActionEvent _component (Utilities|GetNearbyActionStructure))))

(event EventBeginPlay
  (Utilities|FlowControl|Sequence
    (:then_0
      (EventDispatchers|BindEventtoOnNearbyInteractionBegin (delegate Custom|OnNearbyInteractionBeginEvent)))
    (:then_1
      (EventDispatchers|BindEventtoOnNearbyInteractionEnd (delegate Custom|OnNearbyInteractionEndEvent)))))

(fn ConstructionScript)