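; Inventory item actor for a cone pickup that can be interacted with and placed in the inventory.
; The construction script loads the Item_Cone_01 rows from the game item and inventory meta data tables into its GameItem and Inventorable components.
; It then configures the interactable sphere with a Cone prompt of Inventory interaction type, exposed through a getter.
; Inventory item actions only print the actor's name; overlap events are empty.
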(event OnComponentBeginOverlap(BP_InteractableSphereComponent)
  (params (OverlappedComponent :type Primitive%20Component%20Object%20Reference) (OtherActor :type Actor%20Object%20Reference) (OtherComp :type Primitive%20Component%20Object%20Reference) (OtherBodyIndex :type Integer) (bFromSweep :type Boolean) (SweepResult :type Hit%20Result%20Structure%20%28by%20ref%29)))

(event OnComponentEndOverlap(BP_InteractableSphereComponent)
  (params (OverlappedComponent :type Primitive%20Component%20Object%20Reference) (OtherActor :type Actor%20Object%20Reference) (OtherComp :type Primitive%20Component%20Object%20Reference) (OtherBodyIndex :type Integer)))

(event OnInventoryItemAction(BP_InventorableActorComponent)
  (params (InventoryActor :type Actor%20Object%20Reference))
  (Development|PrintString (Utilities|GetDisplayName InventoryActor)))

(event EventBeginPlay)

(event Collision|EventActorBeginOverlap
  (params (OtherActor :type Actor%20Object%20Reference)))

(event EventTick
  (params (DeltaSeconds :type Float%20%28single-precision%29)))

(fn ConstructionScript
  ;[1 1 1] Set GameItem
  (bind _returnvalue (Utilities|GetDataTableRow "/Game/DataTable/DT_GameItemDataTable.DT_GameItemDataTable" "Item_Cone_01")
    (:then
      (Variables|/Script/Sas3.GameItemActorComponent|SetGameItem3 (Variables|Default|GetBP_ActorComponent_GameItem) _returnvalue)
      ;[1 1 1] Set inventory meta
      (bind _returnvalue_2 (Utilities|GetDataTableRow "/Game/DataTable/DP_InventoryMetaDataTable.DP_InventoryMetaDataTable" "Item_Cone_01")
        (:then
          (Variables|/Script/Sas3.InventorableActorComponent|SetInventoryMeta (Variables|Default|GetBP_InventorableActorComponent) _returnvalue_2)
          ;[1 1 1] Set interaction
          (Variables|/Script/Sas3.InteractableSphereComponent|SetInteractionStructure (Variables|Default|GetBP_InteractableSphereComponent) (Utilities|Struct|MakeInteractionStructure "Cone" "Interact with a Cone" "Inventory")))))))

(fn GetInteractableSphereComponent
  (return (Variables|Default|GetBP_InteractableSphereComponent)))