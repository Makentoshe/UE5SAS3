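; An interactable environment actor that loads the game from the current general save slot.
; Starting interaction on its sphere component calls the saveload game instance subsystem to load that slot.
; On BeginPlay it binds to the subsystem's async load started and completed events, printing a message for each.
; It overrides construction functions to supply its "Load Game" title, description and Environment interaction type.
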(event OnInteractionStarted(BP_InteractableSphereComponent)
  (Class|SaveloadGameInstanceSubsystem|LoadCurrentGeneralSaveloadSlot (Subsystems|GetSaveloadGameInstanceSubsystem)))

(event Custom|OnAsyncLoadGameStarted_Event_0
  (params (Structure :type Saveload%20Slot%20Structure%20Structure))
  (Development|PrintString "Loading started"))

(event Custom|OnAsyncLoadGameCompleted_Event_0
  (params (LoadGameGeneral :type Save%20Game%20General%20Object%20Reference))
  (Development|PrintString "Loading completed"))

(event EventBeginPlay
  (EventDispatchers|AssignOnAsyncLoadGameStarted (Subsystems|GetSaveloadGameInstanceSubsystem) (delegate Custom|OnAsyncLoadGameStarted_Event_0))
  (EventDispatchers|AssignOnAsyncLoadGameCompleted (Subsystems|GetSaveloadGameInstanceSubsystem) (delegate Custom|OnAsyncLoadGameCompleted_Event_0)))

(fn ConstructionScript
  (|CallParentFunction))

(fn ConstructionGameItemStructure
  (return (Utilities|Struct|MakeGameItemStructure "Load Game")))

(fn ConstructionInteractionStructure
  (return (Utilities|Struct|MakeInteractionStructure (Utilities|Struct|BreakGameItemStructure (CallFunction|ConstructionGameItemStructure)) "Load game from general slot" "Environment")))