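; BP_Actor_Inventory_Debug is a debug inventory item actor, represented by a cube, that offers a nearby pickup interaction.
; Construction functions build its item, inventory meta and interaction structures, using an item count variable and a fixed stack size.
; The interaction prompt reuses the item title and shows the count, and the cube is exposed as the outlineable mesh.
; The event graph holds only empty placeholder events.
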(event EventBeginPlay)

(event Collision|EventActorBeginOverlap
  (params (OtherActor :type Actor%20Object%20Reference)))

(event EventTick
  (params (DeltaSeconds :type Float%20%28single-precision%29)))

(fn ConstructionScript
  (|CallParentFunction))

(fn ConstructionGameItemStructure
  (return (Utilities|Struct|MakeGameItemStructure "Debug")))

(fn ConstructionInventoryMetaStructure
  (return (Utilities|Struct|MakeInventoryMetaStructure (Variables|Default|GetItemCount) 5)))

(fn ConstructionInteractionStructure
  (return (Utilities|Struct|MakeInteractionStructure (Utilities|Struct|BreakGameItemStructure (CallFunction|ConstructionGameItemStructure)) (Utilities|String|StringToName (Utilities|String|Append "Pick up: " (Utilities|String|ToString(Integer) (.ItemCount (Utilities|Struct|BreakInventoryMetaStructure (CallFunction|ConstructionInventoryMetaStructure)))))) "Inventory")))

(fn GetOutlineableMeshComponents
  (return (Utilities|Array|MakeArray (Variables|Default|GetCube))))