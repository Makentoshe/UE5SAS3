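; Interactable lever actor that broadcasts an event dispatcher when used, leaving the response to whatever binds it.
; Interaction component delegates show a "Lever" display label on selection, hide it on unselection or unavailability, and fire the dispatcher on interact.
; The saveload component re-enables Sphere collision on load unless the actor is saved as destroyed; serialization stores nothing extra.
; Getters expose the interaction and saveload components.
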(event OnInteractionComponentSelectedDelegate(BP_InteractionComponent)
  ;[1 1 1] Display Feature
  (Class|LabelDisplayWidgetComponent|ShowDisplayWidget (Variables|Default|GetBP_DisplayComponent) (Utilities|Struct|MakeSDisplayLabel "Lever")))

(event OnInteractionComponentUnselectedDelegate(BP_InteractionComponent)
  ;[1 1 1] Display Feature
  (Class|DisplayWidgetComponent|HideDisplayWidget (Variables|Default|GetBP_DisplayComponent)))

(event OnInteractionComponentUnavailableDelegate(BP_InteractionComponent)
  ;[1 1 1] Display Feature
  (Class|DisplayWidgetComponent|HideDisplayWidget (Variables|Default|GetBP_DisplayComponent)))

(event OnInteractionComponentInteractDelegate(BP_InteractionComponent)
  (params (InteractorComponent :type Interactor%20Component%20Interface%20%28by%20ref%29))
  ;[1 1 1] Interaction Feature
  (Default|CallNewEventDispatcher))

(event OnSerializeDelegate(BP_SaveloadActorComponent)
  (params (SaveloadObject :type S%20Saveload%20Object%20Structure%20%28by%20ref%29))
  ;[1 1 1] Saveload Feature
)

(event OnDeserializeDelegate(BP_SaveloadActorComponent)
  (params (SaveloadObject :type S%20Saveload%20Object%20Structure%20%28by%20ref%29))
  ;[1 1 1] Saveload Feature
  (if (not (Utilities|Struct|BreakSSaveloadObject SaveloadObject))
    (Collision|SetCollisionEnabled (Variables|Default|GetSphere) "QueryAndPhysics")))

(fn ConstructionScript)

(fn GetInteractionComponent
  (return (Variables|Default|GetBP_InteractionComponent)))

(fn GetSaveloadComponent
  (return (Variables|Default|GetBP_SaveloadActorComponent)))