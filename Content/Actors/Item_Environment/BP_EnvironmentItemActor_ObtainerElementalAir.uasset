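; BP_EnvironmentItemActor_ObtainerElementalAir is an environment item actor, named as an elemental air obtainer, that can be interacted with once.
; The InternalOnGameItemInteracted function swaps the Cube to a gray prototype grid material and sets IsInteracted, while repeat interactions only print a debug message.
; BeginPlay and construction defer to the parent, the nearby interaction event is empty, and no granting of air is implemented here.
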(event Custom|OnNearbyInteractionEvent_1)

(event EventBeginPlay
  (|CallParentFunction))

(fn ConstructionScript
  (|CallParentFunction))

(fn InternalonGameItemInteracted
  (if (Variables|Default|GetIsInteracted?)
    (Development|PrintString "Already interacted")
    (else
      (Utilities|FlowControl|Sequence
        (:then_0
          (Rendering|Material|SetMaterial (Variables|Default|GetCube) 0 "/Game/Prototyping/Greybox/Materials/MI_PrototypeGrid_Gray_Absolute.MI_PrototypeGrid_Gray_Absolute")
          (Variables|Default|SetIsInteracted? true))))))