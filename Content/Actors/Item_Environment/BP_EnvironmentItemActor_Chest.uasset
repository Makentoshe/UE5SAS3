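; Environment item actor for an interactable chest that gives out an inventory item when opened, using a cube as its outlinable mesh.
; The interaction action spawns a sphere inventory item actor with a fixed count at the interactable sphere component's location.
; When the interaction finishes, the chest disables further interaction and swaps the cube to a gray material to look uninteractable.
; Opening animation and VFX are still marked TODO.
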(event OnInteractionAction(BP_InteractableSphereComponent)
  (params (InteractedActor :type Actor%20Object%20Reference) (InteractionWrapper :type Interaction%20Wrapper%20Object%20Reference))
  ;[1 1 1] Chest opening
  ; TODO: Play animation and vfx effects
  (Game|SpawnActorfromClass "/Game/Actors/Item_Inventory/BP_InventoryItemActor_Sphere.BP_InventoryItemActor_Sphere_C" (Math|Transform|MakeTransform (Transformation|GetWorldLocation (Variables|Default|GetBP_InteractableSphereComponent))) "AlwaysSpawn" 0 13 0))

(event OnInteractionFinished(BP_InteractableSphereComponent)
  (params (InteractedActor :type Actor%20Object%20Reference) (InteractionWrapper :type Interaction%20Wrapper%20Object%20Reference))
  ;[1 1 1] Finishing chest opening
  ; Disable interaction with this actor and indicate in uninteractable
  (CallFunction|DisableInteractionforThisActor InteractedActor InteractionWrapper)
  (Rendering|Material|SetMaterial (Variables|Default|GetCube) 0 "/Game/Prototyping/Greybox/Materials/MI_PrototypeGrid_Gray_Relative.MI_PrototypeGrid_Gray_Relative"))

(fn ConstructionScript
  (|CallParentFunction))

(fn GetOutlinableMeshComponents
  (return (Utilities|Array|MakeArray (Variables|Default|GetCube))))