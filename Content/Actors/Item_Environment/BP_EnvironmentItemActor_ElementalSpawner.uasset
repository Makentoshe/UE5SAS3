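; An interactable environment item that grants a companion elemental to whoever interacts with it.
; On interaction, if the actor implements the elemental component holder interface, it reads the hardcoded Nature_Losa creature data table row, wraps it and adds it as a companioning elemental.
; When interaction finishes, it disables further interaction for that actor and switches the cube, also its outlinable mesh, to a gray material.
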(event OnInteractionAction(BP_InteractableSphereComponent)
  (params (InteractedActor :type Actor%20Object%20Reference) (InteractionWrapper :type Interaction%20Wrapper%20Object%20Reference))
  (if (Utilities|DoesObjectImplementInterface InteractedActor "/Game/Features/Feature_Elemental/Interfaces/BPI_Elemental_ActorComponentHolder.BPI_Elemental_ActorComponentHolder_C")
    (bind _component (Class|BPIElementalActorComponentHolder|GetElementalActorComponent(Message) InteractedActor))
    (bind _returnvalue (Utilities|GetDataTableRow "/Game/Characters/Elementales/DataTables/DT_ElementalCreature_DataTable.DT_ElementalCreature_DataTable" "Nature_Losa")
      (:then
        (bind _returnvalue_2 (Game|ConstructObjectfromClass "/Game/Characters/Elementales/Structures/Wrappers/BP_ElementalCreatureWrapper.BP_ElementalCreatureWrapper_C"))
        (Variables|/Game/Characters/Elementales/Structures/Wrappers/BP_ElementalCreatureWrapper.BP_ElementalCreatureWrapper_C|SetElementalCreatureStructure _returnvalue_2 _returnvalue)
        (Default|AddCompanioningElemental _component _returnvalue_2)))))

(event OnInteractionFinished(BP_InteractableSphereComponent)
  (params (InteractedActor :type Actor%20Object%20Reference) (InteractionWrapper :type Interaction%20Wrapper%20Object%20Reference))
  (CallFunction|DisableInteractionforThisActor InteractedActor InteractionWrapper)
  (Rendering|Material|SetMaterial (Variables|Default|GetCube) 0 "/Game/Prototyping/Greybox/Materials/MI_PrototypeGrid_Gray_Relative.MI_PrototypeGrid_Gray_Relative"))

(fn ConstructionScript
  (|CallParentFunction))

(fn GetOutlinableMeshComponents
  (return (Utilities|Array|MakeArray (Variables|Default|GetCube))))