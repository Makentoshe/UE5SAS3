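; BP_EnvironmentItemActor3_SpawnerCube is an interactable environment item that acts as a cube spawner.
; On interaction, it runs the parent logic, then spawns a BP_InventoryItemActor_Cube at its own location with zero rotation and unit scale, ignoring collisions.
; It exposes its BPActorComponentGameItem through GetGameItemActorComponent, while BeginPlay and construction only defer to the parent.
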(event Custom|OnNearbyInteractionEvent_1)

(event EventBeginPlay
  (|CallParentFunction))

(fn ConstructionScript
  (|CallParentFunction))

(fn InternalonGameItemInteracted
  (params (InteractedActor :type Actor%20Object%20Reference))
  (|CallParentFunction 0)
  (Game|SpawnActorfromClass "/Game/Actors/Item_Inventory/BP_InventoryItemActor_Cube.BP_InventoryItemActor_Cube_C" (Math|Transform|MakeTransform (.Location (Math|Transform|BreakTransform (Transformation|GetActorTransform)))) "AlwaysSpawn" 0 0))

(fn GetGameItemActorComponent
  (return (Variables|Default|GetBP_ActorComponent_GameItem)))