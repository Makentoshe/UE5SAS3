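; Interactable world item that grants a fire companion elemental to an interacting actor that implements the elemental component holder interface.
; On interaction it spawns a disabled obtainer at its transform and destroys itself, a workaround for disabling; the nearby-prompt removal is left unconnected.
; It then adds a creature wrapper built from the Mock_Fire_Test data table row to the actor's elemental component and shows it on the HUD as an obtained item.
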(event Custom|OnNearbyInteractionEvent_1)

(event EventBeginPlay
  (|CallParentFunction))

(fn ConstructionScript
  (|CallParentFunction))

(fn InternalonGameItemInteracted
  (params (InteractedActor :type Actor%20Object%20Reference))
  (|CallParentFunction InteractedActor)
  ;[1 1 1] Check is able to interact
  (if (Utilities|DoesObjectImplementInterface InteractedActor "/Game/Features/Feature_Elemental/Interfaces/BPI_Elemental_ActorComponentHolder.BPI_Elemental_ActorComponentHolder_C")
    (Utilities|FlowControl|Sequence
      (:then_0
        ;[0 0 0] Disabling current actor with workaround:
        ; Just add another disabled actor and remove current one
        (Utilities|FlowControl|Sequence
          (:then_0
            ;;[1 1 1] Spawn new disabled actor
            (Game|SpawnActorfromClass "/Game/Actors/Item_Environment/Obtainers/BP_EnvironmentItemActor_ObtainerDisabled.BP_EnvironmentItemActor_ObtainerDisabled_C" (Transformation|GetActorTransform self) "AlwaysSpawn" 0 0))
          (:then_1
            ;;[1 1 1] Remove Interaction ui for the all nearby actors that contains InteractorActorComponent
            (for _array_element (Collision|GetOverlappingActors (Variables|Default|GetInteractionSphereComponent) 0 :!class /Script/Engine.PrimitiveComponent)
              (if (Utilities|DoesObjectImplementInterface _array_element "/Script/Sas3.InteractorActorComponentHolder")
                (bind _returnvalue (Class|InteractorActorComponentHolder|GetInteractorActorComponent(Message) _array_element)))))
          (:then_2
            ;;[1 1 1] Destroy current actor
            (Actor|DestroyActor self))))
      (:then_1
        ;[1 1 1] Add compaioning elemental using ElementalComponent
        (bind _component (Class|BPIElementalActorComponentHolder|GetElementalActorComponent(Message) InteractedActor))
        (bind _returnvalue_2 (Game|ConstructObjectfromClass "/Game/Pawns/Elementales/Structures/Wrappers/BP_ElementalCreatureWrapper.BP_ElementalCreatureWrapper_C"))
        (Utilities|FlowControl|Sequence
          (:then_0
            (bind _returnvalue_3 (Utilities|GetDataTableRow "/Game/DataTable/DT_ElementalCreature_DataTable.DT_ElementalCreature_DataTable" "Mock_Fire_Test")
              (:then
                (bind _output_get (Variables|/Game/Pawns/Elementales/Structures/Wrappers/BP_ElementalCreatureWrapper.BP_ElementalCreatureWrapper_C|SetElementalCreatureStructure _returnvalue_2 _returnvalue_3)))))
          (:then_1
            (Default|AddCompanioningElemental _component _returnvalue_2))))
      (:then_2
        ;[1 1 1] Display obtained compation
        (bind _component_2 (Class|BPICharacterHudActorComponentHolder|GetCharacterHudComponent(Message) InteractedActor))
        (bind _returnvalue_4 (Game|ConstructObjectfromClass "/Script/Sas3.ObtainedItemWrapper"))
        (Utilities|FlowControl|Sequence
          (:then_0
            (Variables|/Script/Sas3.ObtainedItemWrapper|SetObtainedItemStructure _returnvalue_4 (Utilities|Struct|MakeObtainedItemStructure (.Title (Utilities|Struct|BreakElementalCreatureStructure _output_get)) 1 false)))
          (:then_1
            (Default|AddObtainedItem _component_2 _returnvalue_4)))))))