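; Base environment item for an elemental air obtainer that swaps itself for a disabled version when interacted with.
; After the parent interaction logic, it spawns the Disabled actor at its own transform.
; It then removes its nearby-interaction UI entry from every overlapping actor that implements the interactor component holder interface, and destroys itself.
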(event Custom|OnNearbyInteractionEvent_1)

(event EventBeginPlay
  (|CallParentFunction))

(fn ConstructionScript
  (|CallParentFunction))

(fn InternalonGameItemInteracted
  (params (InteractedActor :type Actor%20Object%20Reference))
  (|CallParentFunction 0))

(fn InternalonGameItemInteracted0
  (|CallParentFunction 0)
  (Utilities|FlowControl|Sequence
    (:then_0
      ;[1 1 1] Spawn new disabled actor
      (Game|SpawnActorfromClass "/Game/Actors/Item_Environment/BP_EnvironmentItemActor_ObtainerElementalAir_Disabled.BP_EnvironmentItemActor_ObtainerElementalAir_Disabled_C" (Transformation|GetActorTransform self) "AlwaysSpawn" 0 0))
    (:then_1
      ;[1 1 1] Remove Interaction ui for the selected actor
      (for _array_element (Collision|GetOverlappingActors (Variables|Default|GetInteractionSphereComponent) "/Script/Engine.Actor" :!class /Script/Engine.PrimitiveComponent)
        (if (Utilities|DoesObjectImplementInterface _array_element "/Script/Sas3.InteractorActorComponentHolder")
          (bind _returnvalue (Class|InteractorActorComponentHolder|GetInteractorActorComponent(Message) _array_element))
          (bind _returnvalue_2 (Class|EnvironmentItemActor|BuildNearbyInteractionStructure))
          (Class|InteractorActorComponent|RemoveNearbyInteractionStructure _returnvalue _returnvalue_2))))
    (:then_2
      ;[1 1 1] Destroy current actor
      (Actor|DestroyActor self))))