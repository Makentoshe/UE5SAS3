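; Base actor for environment items that carry game item data and can be interacted with.
; The construction script fills the game item component from the item data table, then builds the interactable sphere's interaction structure from that item's title and the interaction meta table's description.
; A disable function removes the interaction wrapper from the interactor's component via an interface and switches off the sphere's interaction.
; Getters expose both components.
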(fn ConstructionScript
  (Utilities|FlowControl|Sequence
    (:then_0
      ;[1 1 1] Initialize GameItem component
      (bind _returnvalue (Utilities|GetDataTableRow "/Game/Actors/Items/DataTables/DT_GameItemDataTable.DT_GameItemDataTable" (Variables|Item|DataTable|GetGameItemRowName))
        (:then
          (Variables|/Script/Sas3.GameItemActorComponent|SetGameItem3 (Variables|Default|GetBP_ActorComponent_GameItem) _returnvalue))))
    (:then_1
      ;[1 1 1] Initialize InteractableComponent
      (bind _returnvalue_2 (Utilities|GetDataTableRow "/Game/Actors/Items/DataTables/DT_InteractionMetaDataTable.DT_InteractionMetaDataTable" (Variables|Item|DataTable|GetInteractionMetaRowName))
        (:then
          (Variables|/Script/Sas3.InteractableSphereComponent|SetInteractionStructure (Variables|Default|GetBP_InteractableSphereComponent) (Utilities|Struct|MakeInteractionStructure (Utilities|Struct|BreakGameItemStructure (Variables|/Script/Sas3.GameItemActorComponent|GetGameItem3 (Variables|Default|GetBP_ActorComponent_GameItem))) (Utilities|String|StringToName (Utilities|Struct|BreakInteractionMetaStructure _returnvalue_2)) "None")))))))

(fn DisableInteractionforThisActor
  (params (InteractedActor :type Actor%20Object%20Reference) (InteractionWrapper :type Interaction%20Wrapper%20Object%20Reference))
  (if (Utilities|DoesObjectImplementInterface InteractedActor "/Script/Sas3.InteractorActorComponentHolder")
    (bind _returnvalue (Class|InteractorActorComponentHolder|GetInteractorActorComponent(Message) InteractedActor))
    (Class|InteractorActorComponent|RemoveInteractionWrapper _returnvalue InteractionWrapper)
    (Variables|/Script/Sas3.InteractableSphereComponent|SetIsInteractionEnabled (Variables|Default|GetBP_InteractableSphereComponent) false)))

(fn GetGameItemActorComponent
  (return (Variables|Default|GetBP_ActorComponent_GameItem)))

(fn GetInteractableSphereComponent
  (return (Variables|Default|GetBP_InteractableSphereComponent)))