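; Base actor for interactable game items, pairing a game item component with an interactable sphere component.
; The construction script fills both components from structure functions that are empty here, as is the outlineable mesh getter.
; Sphere selection events toggle custom depth on those meshes for outlining.
; Add and remove events pass an InteractionWrapper to the interactor's component through an interface, keeping components decoupled.
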(event OnInteractionSelectedChanged(BP_InteractableSphereComponent)
  (params (InteractedActor :type Actor%20Object%20Reference) (IsActorSelected :type Boolean))
  ;[1 1 1] Invokes when item should indicate its selection
  (for _array_element (Interaction|GetOutlineableMeshComponents)
    (Rendering|SetRenderCustomDepth _array_element IsActorSelected)))

(event OnRemoveInteractionWrapper(BP_InteractableSphereComponent)
  (params (InteractorActor :type Actor%20Object%20Reference) (Structure :type Interaction%20Structure%20Structure))
  ;[1 0.848 0 0.5] Components communication:
  ; Event from one component invokes method of the other
  ;;[1 1 1] Interaction
  ;; Check is Actor is able to Interact and ask it to remove it from available interactions list
  (if (Utilities|DoesObjectImplementInterface InteractorActor "/Script/Sas3.InteractorActorComponentHolder")
    (bind _returnvalue (Class|InteractorActorComponentHolder|GetInteractorActorComponent(Message) InteractorActor))
    (Class|InteractorActorComponent|RemoveInteractionWrapper _returnvalue (Variables|Default|GetInteractionWrapper))))

(event OnAddInteractionWrapper(BP_InteractableSphereComponent)
  (params (InteractorActor :type Actor%20Object%20Reference) (Structure :type Interaction%20Structure%20Structure))
  ;[1 0.848 0 0.5] Components communication:
  ; Event from one component invokes method of the other
  ;;[1 1 1] Interaction
  ;; Check is Actor is able to Interact and ask it to add it to available interactions list
  (if (Utilities|DoesObjectImplementInterface InteractorActor "/Script/Sas3.InteractorActorComponentHolder")
    (bind _returnvalue (Class|InteractorActorComponentHolder|GetInteractorActorComponent(Message) InteractorActor))
    (bind _returnvalue_2 (Game|ConstructObjectfromClass "/Script/Sas3.InteractionWrapper" Structure (Variables|Default|GetBP_InteractableSphereComponent)))
    (bind _output_get (Variables|Default|SetInteractionWrapper _returnvalue_2))
    (Class|InteractorActorComponent|AddInteractionWrapper _returnvalue _output_get)))

(fn ConstructionScript
  (Variables|/Script/Sas3.GameItemActorComponent|SetGameItem3 (Variables|Default|GetBP_ActorComponent_GameItem) (Construction|ConstructionGameItemStructure))
  (Variables|/Script/Sas3.InteractableSphereComponent|SetInteractionStructure (Variables|Default|GetBP_InteractableSphereComponent) (Construction|ConstructionInteractionStructure)))

(fn ConstructionGameItemStructure
  (return ""))

(fn ConstructionInteractionStructure
  (return ""))

(fn GetOutlineableMeshComponents
  (return 0))

(fn GetGameItemActorComponent
  (return (Variables|Default|GetBP_ActorComponent_GameItem)))

(fn GetInteractableSphereComponent
  (return (Variables|Default|GetBP_InteractableSphereComponent)))