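; Base actor for inventory items that lie in the world and are picked up by interaction.
; The construction script fills the game item and inventory meta components from two data tables by RowName, overriding the item count.
; It then builds the interactable sphere's prompt from the item title and count.
; The actor destroys itself when interaction finishes, prints interaction issues, and exposes getters for its three components.
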(event OnInteractionFinished(BP_InteractableSphereComponent)
  (params (InteractedActor :type Actor%20Object%20Reference) (InteractionWrapper :type Interaction%20Wrapper%20Object%20Reference))
  ;[1 1 1] When interaction finished - actor can be destroyed
  ; Because it is inventory item and after interaction it should be "placed" in the player's inventory
  (Actor|DestroyActor))

(event OnComponentIssues(BP_InteractableSphereComponent)
  (params (Reason :type EInteractableComponentIssues%20Enum :default "InteractionOverlapInterface"))
  ;[1 0 0 0.5] Handle issues
  (Development|PrintString (Utilities|String|EnumtoString Reason) true true "(R=1.000000,G=0.000000,B=0.000000,A=1.000000)" 1.0))

(event OnInteractionAction(BP_InteractableSphereComponent)
  (params (InteractedActor :type Actor%20Object%20Reference) (InteractionWrapper :type Interaction%20Wrapper%20Object%20Reference))
  ;[1 1 1] Invokes when item should do any action
)

(fn ConstructionScript
  (Utilities|FlowControl|Sequence
    (:then_0
      (bind _returnvalue (Utilities|GetDataTableRow "/Game/Actors/Items/DataTables/DT_GameItemDataTable.DT_GameItemDataTable" (Variables|Item|DataTable|GetRowName))
        (:then
          (Variables|/Script/Sas3.GameItemActorComponent|SetGameItem3 (Variables|Default|GetBP_ActorComponent_GameItem) _returnvalue))))
    (:then_1
      (bind _returnvalue_2 (Utilities|GetDataTableRow "/Game/DataTable/DP_InventoryMetaDataTable.DP_InventoryMetaDataTable" (Variables|Item|DataTable|GetRowName))
        (:then
          (bind _structout (Utilities|Struct|SetmembersinInventoryMetaStructure _returnvalue_2 (Variables|Item|GetItemCount)))
          (Variables|/Script/Sas3.InventorableActorComponent|SetInventoryMeta (Variables|Default|GetBP_InventorableActorComponent) _structout))))
    (:then_2
      (Variables|/Script/Sas3.InteractableSphereComponent|SetInteractionStructure (Variables|Default|GetBP_InteractableSphereComponent) (Utilities|Struct|MakeInteractionStructure (Utilities|Struct|BreakGameItemStructure (Variables|/Script/Sas3.GameItemActorComponent|GetGameItem3 (Variables|Default|GetBP_ActorComponent_GameItem))) (Utilities|String|StringToName (Utilities|String|Append "Pick up: " (Utilities|String|ToString(Integer) (.ItemCount (Utilities|Struct|BreakInventoryMetaStructure (Variables|/Script/Sas3.InventorableActorComponent|GetInventoryMeta (Variables|Default|GetBP_InventorableActorComponent))))))) "None")))))

(fn GetGameItemActorComponent
  (return (Variables|Default|GetBP_ActorComponent_GameItem)))

(fn GetInteractableSphereComponent
  (return (Variables|Default|GetBP_InteractableSphereComponent)))

(fn GetInventorableActorComponent
  (return (Variables|Default|GetBP_InventorableActorComponent)))