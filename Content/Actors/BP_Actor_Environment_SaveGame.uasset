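; BP_Actor_Environment_SaveGame is an interactable environment actor that saves the game to the current general save slot.
; Starting an interaction on its sphere component calls the saveload game instance subsystem to save.
; On BeginPlay it binds to the subsystem's async save started and completed events, which only print status messages.
; Construction functions supply its "Save Game" item title and interaction prompt.
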(event OnInteractionStarted(BP_InteractableSphereComponent)
  (Class|SaveloadGameInstanceSubsystem|SaveCurrentGeneralSaveloadSlot (Subsystems|GetSaveloadGameInstanceSubsystem)))

(event Custom|OnAsyncSaveGameStarted_Event_0
  (params (Structure :type Saveload%20Slot%20Structure%20Structure) (SaveGameGeneral :type Save%20Game%20General%20Object%20Reference))
  (Development|PrintString "Saving started"))

(event Custom|OnAsyncSaveGameCompleted_Event_0
  (params (SlotName :type String) (UserIndex :type Integer) (bSuccess :type Boolean))
  (Development|PrintString "Saving completed"))

(event EventBeginPlay
  (EventDispatchers|AssignOnAsyncSaveGameStarted (Subsystems|GetSaveloadGameInstanceSubsystem) (delegate Custom|OnAsyncSaveGameStarted_Event_0))
  (EventDispatchers|AssignOnAsyncSaveGameCompleted (Subsystems|GetSaveloadGameInstanceSubsystem) (delegate Custom|OnAsyncSaveGameCompleted_Event_0)))

(fn ConstructionScript
  (|CallParentFunction))

(fn ConstructionGameItemStructure
  (return (Utilities|Struct|MakeGameItemStructure "Save Game")))

(fn ConstructionInteractionStructure
  (return (Utilities|Struct|MakeInteractionStructure (Utilities|Struct|BreakGameItemStructure (CallFunction|ConstructionGameItemStructure)) "Save game to general slot" "Environment")))