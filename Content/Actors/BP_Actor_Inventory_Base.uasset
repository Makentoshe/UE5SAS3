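; Base actor for world items that the player picks up into an inventory.
; Its construction script fills the inventorable component from ConstructionInventoryMetaStructure, which is empty here.
; The component's inventory action builds an item from that construction metadata and the game item title, then adds it to the given inventory.
; Finished interaction hides the actor, disables collision and zeroes its count rather than destroying it, and a counterpart function restores it with a given count.
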(event OnInventoryItemAction(BP_InventorableActorComponent)
  (params (InventoryComponent :type Inventory%20Actor%20Component%20Object%20Reference))
  (bind _inventorymetastructure (Construction|ConstructionInventoryMetaStructure))
  (bind (_itemcount _stacksize) (Utilities|Struct|BreakInventoryMetaStructure _inventorymetastructure))
  ;[1 1 1] Inventory - Inventory action called
  ; We need to compose InventoryWrapper and add it to the InventoryComponent
  (Class|InventoryActorComponent|AddInventoryItem InventoryComponent (Utilities|Struct|MakeInventoryItemStructure _itemcount _stacksize (Utilities|Struct|BreakGameItemStructure (CallFunction|ConstructionGameItemStructure)))))

(event OnInteractionFinished(BP_InteractableSphereComponent)
  ;[1 1 1] When interaction finished - actor can be removed
  ; Because it is inventory item and after interaction it should be "placed" in the player's inventory
  (CallFunction|DisableInteractionDueInventoryPickup))

(fn ConstructionScript
  (|CallParentFunction)
  (Variables|/Script/Sas3.InventorableActorComponent|SetInventoryMeta (Variables|Default|GetBP_InventorableActorComponent) (Construction|ConstructionInventoryMetaStructure)))

(fn ConstructionInventoryMetaStructure
  (return ""))

(fn DisableInteractionDueInventoryPickup
  (Rendering|SetActorHiddenInGame true)
  (Collision|SetActorEnableCollision self false)
  (bind _returnvalue (CallFunction|GetInventorableActorComponent))
  (Variables|/Script/Sas3.InventorableActorComponent|SetInventoryMeta _returnvalue (Utilities|Struct|MakeInventoryMetaStructure 0 (Utilities|Struct|BreakInventoryMetaStructure (Variables|/Script/Sas3.InventorableActorComponent|GetInventoryMeta _returnvalue)))))

(fn EnableInteractionDueInventoryPickup
  (params (Item%20Count :type Integer))
  (Rendering|SetActorHiddenInGame false)
  (Collision|SetActorEnableCollision self true)
  (bind _returnvalue (CallFunction|GetInventorableActorComponent))
  (Variables|/Script/Sas3.InventorableActorComponent|SetInventoryMeta _returnvalue (Utilities|Struct|MakeInventoryMetaStructure Item%20Count (Utilities|Struct|BreakInventoryMetaStructure (Variables|/Script/Sas3.InventorableActorComponent|GetInventoryMeta _returnvalue)))))

(fn GetInventorableActorComponent
  (return (Variables|Default|GetBP_InventorableActorComponent)))