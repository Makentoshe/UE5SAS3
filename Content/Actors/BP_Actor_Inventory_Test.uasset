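; BP_Actor_Inventory_Test is a test inventory pickup that represents a cube item with a randomized item count.
; It overrides construction functions that pull item and inventory data from data tables, inject the count, and build a "Pick up" interaction prompt.
; When the saveload component deserializes it, it restores the count, then disables pickup interaction if empty or rebuilds and enables it.
; The cube mesh is exposed for outlining.
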(event OnActorDeserialized(BP_ActorComponent_Saveloadable)
  (params (Structure :type Saveload%20Actor%20Structure%20Structure))
  ;[1 1 1] Saveload
  ; When actor was deserialized - restore it state
  (Variables|Default|SetItemsCount (Utilities|Struct|BreakInventorableComponentSaveload (.InventorableComponentSaveload (Utilities|Struct|BreakSaveloadActorStructure Structure))))
  (if (<= (Variables|Default|GetItemsCount) 0)
    (CallFunction|DisableInteractionDueInventoryPickup)
    (else
      (Variables|/Script/Sas3.InteractableSphereComponent|SetInteractionStructure (Variables|Default|GetBP_InteractableSphereComponent) (CallFunction|ConstructionInteractionStructure))
      (CallFunction|EnableInteractionDueInventoryPickup (Variables|Default|GetItemsCount)))))

(fn ConstructionScript
  (Variables|Default|SetItemsCount (Math|Random|RandomInteger 64))
  (|CallParentFunction))

(fn ConstructionGameItemStructure
  (bind _returnvalue (Utilities|GetDataTableRow "/Game/Features/Features/DataTables/DT_GameItemDataTable.DT_GameItemDataTable" "Item_Cube_01")
    (:then
      (return _returnvalue))))

(fn ConstructionInteractionStructure
  (return (Utilities|Struct|MakeInteractionStructure (Utilities|Struct|BreakGameItemStructure (CallFunction|ConstructionGameItemStructure)) (Utilities|String|StringToName (Utilities|String|Append "Pick up: " (Utilities|String|ToString(Integer) (Utilities|Struct|BreakInventoryMetaStructure (CallFunction|ConstructionInventoryMetaStructure))))) "Inventory")))

(fn ConstructionInventoryMetaStructure
  (bind _returnvalue (Utilities|GetDataTableRow "/Game/Features/Feature_Inventory/DataTables/DT_InventoryMetaDataTable.DT_InventoryMetaDataTable" "Item_Cube_01")
    (:then
      (bind _structout (Utilities|Struct|SetmembersinInventoryMetaStructure _returnvalue (Variables|Default|GetItemsCount)))
      (return _structout))))

(fn GetOutlineableMeshComponents
  (return (Utilities|Array|MakeArray (Variables|Default|GetCube))))

(fn GetSaveloadableActorComponent
  (return (Variables|Default|GetBP_ActorComponent_Saveloadable)))