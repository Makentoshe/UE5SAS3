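; An interactable environment actor that starts a battle by switching to the Battle level.
; Interacting flags the actor, then creates and saves a temporary save slot through the SaveloadGameInstanceSubsystem.
; The level opens only when the async save-completed callback reports success and the flag is set.
; It supplies "Begin battle" prompt data and prints debug strings as interactors are added or removed.
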(event OnInteractionStarted(BP_InteractableSphereComponent)
  (bind _returnvalue (Subsystems|GetSaveloadGameInstanceSubsystem))
  (Variables|Default|SetIsInteracted true)
  (Class|SaveloadGameInstanceSubsystem|CreateCurrentTemporalSaveload _returnvalue)
  (Class|SaveloadGameInstanceSubsystem|SaveCurrentTemporalSaveloadSlot _returnvalue))

(event OnAddInteractionWrapper(BP_InteractableSphereComponent)
  (params (InteractorActor :type Actor%20Object%20Reference) (Structure :type Interaction%20Structure%20Structure))
  (Development|PrintString (Utilities|String|Append "begin " (Utilities|GetDisplayName InteractorActor))))

(event OnRemoveInteractionWrapper(BP_InteractableSphereComponent)
  (params (InteractorActor :type Actor%20Object%20Reference) (Structure :type Interaction%20Structure%20Structure))
  (Development|PrintString (Utilities|String|Append "End " (Utilities|GetDisplayName InteractorActor))))

(event Custom|OnAsyncSaveGameCompleted_Event_0
  (params (SlotName :type String) (UserIndex :type Integer) (bSuccess :type Boolean))
  (if (and bSuccess (Variables|Default|GetIsInteracted))
    (Game|OpenLevel(byObjectReference) "/Game/Landscape/Battle/Battle.Battle")))

(event EventBeginPlay
  (EventDispatchers|AssignOnAsyncSaveGameCompleted (Subsystems|GetSaveloadGameInstanceSubsystem) (delegate Custom|OnAsyncSaveGameCompleted_Event_0)))

(fn ConstructionScript
  (|CallParentFunction))

(fn ConstructionGameItemStructure
  (return (Utilities|Struct|MakeGameItemStructure "Begin battle")))

(fn ConstructionInteractionStructure
  (return (Utilities|Struct|MakeInteractionStructure (Utilities|Struct|BreakGameItemStructure (CallFunction|ConstructionGameItemStructure)) "Change level and return back" "Environment")))