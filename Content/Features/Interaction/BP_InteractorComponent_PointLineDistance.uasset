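; Interactor component that picks which available interaction component is selected, based on where a forward ray points.
; Each tick it line-traces from a start component supplied through LateInitialize, then selects the candidate whose owner is closest to the trace segment.
; Candidates projected outside the viewport are skipped, and every non-selected one is told it is unselected.
; The interacted event is only a debug-print placeholder.
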(event EventTick
  (params (DeltaSeconds :type Float%20%28single-precision%29))
  ;[1 1 1] Each tick cast a ray and find nearest available InteractionComponent and select it. And unselect other components
  ; TODO: Move to CPP
  (if (Utilities|Array|IsNotEmpty (Variables|Default|GetAvailableInteractionComponents))
    (bind _outhit (CallFunction|CastRayForwardfromComponentPosition (Variables|Interaction|GetRayCastingStartComponent)))
    (bind _component (CallFunction|GetNearestInteractionComponent (Variables|Default|GetAvailableInteractionComponents) _outhit))
    (bind _output_get (Variables|Default|SetSelectedInteractionComponent _component))
    (for _array_element (Variables|Default|GetAvailableInteractionComponents)
      (if (== (Utilities|ToObject(Interface) _output_get) (Utilities|ToObject(Interface) _array_element))
        (Class|InteractionComponent|OnInteractionComponentSelected _array_element)
        (else
          (Class|InteractionComponent|OnInteractionComponentUnselected _array_element))))
    (else
      (Variables|Default|SetSelectedInteractionComponent 0))))

(event EventOnInteractionComponentInteracted
  (params (Component :type Interaction%20Component%20Interface%20%28by%20ref%29))
  ;[1 1 1] Character Interacted with OwnerActor
  (Development|PrintString "Do something in BP_InteractorComponent"))

(fn LateInitialize
  (params (Component%20For%20raycasting%20start%20position :type Scene%20Component%20Object%20Reference) (PlayerController :type Player%20Controller%20Object%20Reference))
  (Variables|Interaction|SetRayCastingStartComponent Component%20For%20raycasting%20start%20position)
  (Variables|Interaction|SetPlayerControllerOwner PlayerController))

(fn CastRayForwardfromComponentPosition
  (params (Component :type Scene%20Component%20Object%20Reference))
  (bind _returnvalue (Transformation|GetWorldLocation Component))
  (bind _outhit (Collision|LineTraceByChannel _returnvalue (+ _returnvalue (* (Math|Vector|GetForwardVector Component) 2147483647)) "TraceTypeQuery1" false 0 "ForOneFrame"))
  (return _outhit))

(fn GetNearestInteractionComponent
  (params (Components2 :type Array%20of%20Interaction%20Component%20Interfaces) (LineTraceHit :type Hit%20Result%20Structure))
  (bind (_bblockinghit _binitialoverlap _time _distance _location _impactpoint _normal _impactnormal _physmat _hitactor _hitcomponent _hitbonename _bonename _hititem _elementindex _faceindex _tracestart _traceend) (Collision|BreakHitResult LineTraceHit))
  (bind _returnvalue (Viewport|GetViewportSize))
  (bind (_x _y) (Math|Vector2D|BreakVector2D _returnvalue))
  ;[1 1 1] Setup traces
  (Utilities|FlowControl|Sequence
    (:then_0
      (LocalVariables|SetTraceStartLocation _tracestart)
      (if _binitialoverlap
        (LocalVariables|SetTraceEndLocation _location)
        (else
          (LocalVariables|SetTraceEndLocation _traceend))))
    (:then_1
      (for _array_element Components2
        (bind _asactor_component (Utilities|Casting|CastToActorComponent (Utilities|ToObject(Interface) _array_element))) ; We cast to ActorComponent because we sure \nthat IInteractionComponent will contain only ActorComponent refrence
        (if (or (not (.ReturnValue (Class|PlayerController|ProjectWorldLocationtoScreen (Variables|Interaction|GetPlayerControllerOwner) (Transformation|GetActorLocation (Components|GetOwner _asactor_component)) false))) (Math|Boolean|ANDBoolean (> (.X (Math|Vector2D|BreakVector2D (.ScreenLocation (Class|PlayerController|ProjectWorldLocationtoScreen (Variables|Interaction|GetPlayerControllerOwner) (Transformation|GetActorLocation (Components|GetOwner _asactor_component)) false)))) 0.0) (> (.Y (Math|Vector2D|BreakVector2D (.ScreenLocation (Class|PlayerController|ProjectWorldLocationtoScreen (Variables|Interaction|GetPlayerControllerOwner) (Transformation|GetActorLocation (Components|GetOwner _asactor_component)) false)))) 0.0) (< (.X (Math|Vector2D|BreakVector2D (.ScreenLocation (Class|PlayerController|ProjectWorldLocationtoScreen (Variables|Interaction|GetPlayerControllerOwner) (Transformation|GetActorLocation (Components|GetOwner _asactor_component)) false)))) _x) (< (.Y (Math|Vector2D|BreakVector2D (.ScreenLocation (Class|PlayerController|ProjectWorldLocationtoScreen (Variables|Interaction|GetPlayerControllerOwner) (Transformation|GetActorLocation (Components|GetOwner _asactor_component)) false)))) _y))) ; Check component owner is on the screen\nIf false: skip component
          (if (< (Class|KismetMathLibrary|GetPointDistancetoSegment (Transformation|GetActorLocation (Components|GetOwner _asactor_component)) (LocalVariables|GetTraceStartLocation) (LocalVariables|GetTraceEndLocation)) (LocalVariables|GetNearestSceneComponentLength))
            (LocalVariables|SetNearestSceneComponent2 _array_element)
            (LocalVariables|SetNearestSceneComponentLength (Class|KismetMathLibrary|GetPointDistancetoSegment (Transformation|GetActorLocation (Components|GetOwner _asactor_component)) (LocalVariables|GetTraceStartLocation) (LocalVariables|GetTraceEndLocation))))))
      (return (LocalVariables|GetNearestSceneComponent2)))))