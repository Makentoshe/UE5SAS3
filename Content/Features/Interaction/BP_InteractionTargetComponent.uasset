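; BP_InteractionTargetComponent is a collision component that makes itself known as an interaction target to actors that overlap it.
; On BeginPlay it binds its own begin and end overlap events.
; When the overlapping actor implements BPI_InteractionTriggerComponentHolder, it fetches that actor's trigger component through the interface.
; It adds itself to that trigger component on begin overlap and removes itself on end overlap.
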(event Custom|OnComponentBeginOverlap_Event
  (params (OverlappedComponent :type Primitive%20Component%20Object%20Reference) (OtherActor :type Actor%20Object%20Reference) (OtherComp :type Primitive%20Component%20Object%20Reference) (OtherBodyIndex :type Integer) (bFromSweep :type Boolean) (SweepResult :type Hit%20Result%20Structure%20%28by%20ref%29))
  (if (Utilities|DoesObjectImplementInterface OtherActor "/Game/Features/Interaction/BPI_InteractionTriggerComponentHolder.BPI_InteractionTriggerComponentHolder_C")
    (bind _component (Class|BPIInteractionTriggerComponentHolder|GetInteractionTriggerComponent(Message) OtherActor))
    (Default|AddInteractionTargetComponent _component self)))

(event Custom|OnComponentEndOverlap_Event
  (params (OverlappedComponent :type Primitive%20Component%20Object%20Reference) (OtherActor :type Actor%20Object%20Reference) (OtherComp :type Primitive%20Component%20Object%20Reference) (OtherBodyIndex :type Integer))
  (if (Utilities|DoesObjectImplementInterface OtherActor "/Game/Features/Interaction/BPI_InteractionTriggerComponentHolder.BPI_InteractionTriggerComponentHolder_C")
    (bind _component (Class|BPIInteractionTriggerComponentHolder|GetInteractionTriggerComponent(Message) OtherActor))
    (Default|RemoveInteractionTargetComponent _component self)))

(event EventBeginPlay
  (Utilities|FlowControl|Sequence
    (:then_0
      (Collision|AssignOnComponentBeginOverlap (delegate Custom|OnComponentBeginOverlap_Event)))
    (:then_1
      (Collision|AssignOnComponentEndOverlap (delegate Custom|OnComponentEndOverlap_Event)))))