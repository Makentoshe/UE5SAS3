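; Interaction strategy that picks which interaction component the player targets, based on closeness to a line of sight.
; It line-traces on Visibility along LineTraceComponent's forward vector, ending the segment at the blocking hit or the trace's far end.
; Candidates whose owner location passes a screen-bounds check are compared by point-to-segment distance, and the nearest is returned.
; The screen check also passes locations that fail to project.
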(fn GetInteractorComponent
  (params (Components :type Array%20of%20Interaction%20Component%20Interfaces))
  (bind _tracehit (CallFunction|TraceLinetoForward))
  ;[1 1 1] Setup local variables for trace info
  (Utilities|FlowControl|Sequence
    (:then_0
      (LocalVariables|SetTraceStartLocation (.TraceStart (Collision|BreakHitResult _tracehit)))
      (if (.bBlockingHit (Collision|BreakHitResult _tracehit))
        (LocalVariables|SetTraceEndLocation (.Location (Collision|BreakHitResult _tracehit)))
        (else
          (LocalVariables|SetTraceEndLocation (.TraceEnd (Collision|BreakHitResult _tracehit))))))
    (:then_1
      (for _array_element Components
        (bind _ownerlocation (CallFunction|GetInteractionComponentOwnerLocation _array_element))
        (if (CallFunction|CheckWorldLocationIsontheScreen _ownerlocation)
          (if (< (Class|KismetMathLibrary|GetPointDistancetoSegment _ownerlocation (LocalVariables|GetTraceStartLocation) (LocalVariables|GetTraceEndLocation)) (LocalVariables|GetNearestSceneComponentLength))
            (LocalVariables|SetNearestSceneComponent _array_element)
            (LocalVariables|SetNearestSceneComponentLength (Class|KismetMathLibrary|GetPointDistancetoSegment _ownerlocation (LocalVariables|GetTraceStartLocation) (LocalVariables|GetTraceEndLocation))))))
      (return (LocalVariables|GetNearestSceneComponent)))))

(fn TraceLinetoForward
  (bind _linetracecomponent (Variables|Default|GetLineTraceComponent))
  (bind _returnvalue (Transformation|GetWorldLocation _linetracecomponent))
  (bind _outhit (Class|InteractorStrategy|LineTracebyChannel _returnvalue (+ _returnvalue (* (Math|Vector|GetForwardVector _linetracecomponent) 2147483647)) "ECC_Visibility"))
  (return _outhit))

(fn GetInteractionComponentOwnerLocation
  (params (Component :type Interaction%20Component%20Interface))
  (bind _asactor_component (Utilities|Casting|CastToActorComponent (Utilities|ToObject(Interface) Component))) ; We cast to ActorComponent because we sure \nthat IInteractionComponent will contain only ActorComponent refrence
  (return (Transformation|GetActorLocation (Components|GetOwner _asactor_component))))

(fn CheckWorldLocationIsontheScreen
  (params (WorldLocation :type Vector))
  (bind _playercontrollerowner (Variables|Components|GetPlayerControllerOwner))
  (bind _playercontrollerowner_2 (Variables|Components|GetPlayerControllerOwner))
  (bind (_sizex _sizey) (HUD|GetViewportSize _playercontrollerowner_2))
  (bind (_screenlocation _returnvalue) (Class|PlayerController|ProjectWorldLocationtoScreen _playercontrollerowner WorldLocation false))
  (bind (_x _y) (Math|Vector2D|BreakVector2D _screenlocation))
  (return (or (not _returnvalue) (Math|Boolean|ANDBoolean (> _x 0.0) (> _y 0.0) (< _x _sizex) (< _y _sizey)))))