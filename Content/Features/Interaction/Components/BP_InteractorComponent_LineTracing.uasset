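; Interactor component that picks which available interaction component is selected, based on where a forward line trace lands.
; Each tick it traces on Visibility from a start component supplied through Initialize, drawing debug for one frame.
; It selects the component whose owner is closest to the hit location, first sending unselect to all available components.
; The interacted event only prints placeholder text, and the angle helper is unused here.
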(event EventTick
  (params (DeltaSeconds :type Float%20%28single-precision%29))
  ;[1 1 1] Each tick cast a ray and find nearest available InteractionComponent and select it. And unselect other components
  ; TODO: Move to CPP
  (if (Utilities|Array|IsNotEmpty (Variables|Default|GetAvailableInteractionComponents))
    (bind _outhit (MoveToSubsystem|CastRayForwardfromComponentPosition (Variables|Interaction|GetRayCastingStartComponent)))
    (bind _component2 (MoveToSubsystem|GetNearesttoWorldLocationSceneComponent (.Location (Collision|BreakHitResult _outhit)) (Variables|Default|GetAvailableInteractionComponents)))
    (bind _output_get (Variables|Default|SetSelectedInteractionComponent _component2))
    (for _array_element (Variables|Default|GetAvailableInteractionComponents)
      (Class|InteractionComponent|OnInteractionComponentUnselected _array_element))
    (Class|InteractionComponent|OnInteractionComponentSelected _output_get)
    (else
      (Variables|Default|SetSelectedInteractionComponent 0))))

(event EventOnInteractionComponentInteracted
  (params (Component :type Interaction%20Component%20Interface%20%28by%20ref%29))
  ;[1 1 1] Character Interacted with OwnerActor
  (Development|PrintString "Do something in BP_InteractorComponent"))

(fn GetAngleBetweenSceneComponents
  (params (ComponentTo :type Scene%20Component%20Object%20Reference) (ComponentFrom :type Scene%20Component%20Object%20Reference))
  (return (Class|KismetMathLibrary|DegAcos (Math|Vector|DotProduct (Math|Vector|GetForwardVector ComponentFrom) (Math|Vector|Normalize (- (Transformation|GetWorldLocation ComponentTo) (Transformation|GetWorldLocation ComponentFrom)))))))

(fn GetNearesttoWorldLocationSceneComponent
  (params (WorldLocation :type Vector) (Components2 :type Array%20of%20Interaction%20Component%20Interfaces))
  (for _array_element Components2
    (bind _asactor_component (Utilities|Casting|CastToActorComponent (Utilities|ToObject(Interface) _array_element))) ; We cast to ActorComponent because we sure \nthat IInteractionComponent will contain only ActorComponent refrence
    (if (< (Math|Vector|VectorLength (- (Transformation|GetActorLocation (Components|GetOwner _asactor_component)) WorldLocation)) (LocalVariables|GetNearestSceneComponentLength))
      (LocalVariables|SetNearestSceneComponentLength (Math|Vector|VectorLength (- (Transformation|GetActorLocation (Components|GetOwner _asactor_component)) WorldLocation)))
      (LocalVariables|SetNearestSceneComponent2 _array_element)))
  (return (LocalVariables|GetNearestSceneComponent2)))

(fn Initialize
  (params (Component%20For%20raycasting%20start%20position :type Scene%20Component%20Object%20Reference))
  (Variables|Interaction|SetRayCastingStartComponent Component%20For%20raycasting%20start%20position))

(fn CastRayForwardfromComponentPosition
  (params (Component :type Scene%20Component%20Object%20Reference))
  (bind _returnvalue (Transformation|GetWorldLocation Component))
  (bind _outhit (Collision|LineTraceByChannel _returnvalue (+ _returnvalue (* (Math|Vector|GetForwardVector Component) 1000)) "TraceTypeQuery1" false 0 "ForOneFrame"))
  (return _outhit))