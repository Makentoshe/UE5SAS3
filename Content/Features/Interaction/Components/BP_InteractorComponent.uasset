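; Actor component that tracks nearby or registered interaction components and decides which one is active for interaction.
; Components are added and removed through events that notify each one.
; While any are registered, Tick traces forward on Visibility from a start component set by Initialize, disables all candidates, then enables the one whose owner is nearest the hit location.
; An angle helper exists but is not called here.
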(event EventRemoveInteractionComponent2
  (params (Component :type BPI%20Interaction%20Component%20Interface))
  (Utilities|Array|RemoveItem (Variables|Interaction|GetInteractionComponents2) Component)
  (Default|OnInteractionComponentRemoved Component))

(event EventTick
  (params (DeltaSeconds :type Float%20%28single-precision%29))
  (if (Utilities|Array|IsNotEmpty (Variables|Interaction|GetInteractionComponents2))
    (bind _outhit (MoveToSubsystem|CastRayForwardfromComponentPosition (Variables|Interaction|GetRayCastingStartComponent)))
    (bind _component2 (MoveToSubsystem|GetNearesttoWorldLocationSceneComponent (.Location (Collision|BreakHitResult _outhit)) (Variables|Interaction|GetInteractionComponents2)))
    (for _array_element (Variables|Interaction|GetInteractionComponents2)
      (Default|OnInteractionComponentDisabled _array_element))
    (Default|OnInteractionComponentEnabled _component2)))

(event EventAddInteractionComponent2
  (params (Component :type BPI%20Interaction%20Component%20Interface))
  (Utilities|Array|Add (Variables|Interaction|GetInteractionComponents2) Component)
  (Default|OnInteractionComponentAdded Component))

(fn GetAngleBetweenSceneComponents
  (params (ComponentTo :type Scene%20Component%20Object%20Reference) (ComponentFrom :type Scene%20Component%20Object%20Reference))
  (return (Class|KismetMathLibrary|DegAcos (Math|Vector|DotProduct (Math|Vector|GetForwardVector ComponentFrom) (Math|Vector|Normalize (- (Transformation|GetWorldLocation ComponentTo) (Transformation|GetWorldLocation ComponentFrom)))))))

(fn GetNearesttoWorldLocationSceneComponent
  (params (WorldLocation :type Vector) (Components2 :type Array%20of%20BPI%20Interaction%20Component%20Interfaces))
  (for _array_element Components2
    (bind _location (Default|GetWorldLocationfromOwnerActor _array_element))
    (if (< (Math|Vector|VectorLength (- _location WorldLocation)) (LocalVariables|GetNearestSceneComponentLength))
      (LocalVariables|SetNearestSceneComponentLength (Math|Vector|VectorLength (- _location WorldLocation)))
      (LocalVariables|SetNearestSceneComponent2 _array_element)))
  (return (LocalVariables|GetNearestSceneComponent2)))

(fn Initialize
  (params (Component%20For%20raycasting%20start%20position :type Scene%20Component%20Object%20Reference))
  (Variables|Interaction|SetRayCastingStartComponent Component%20For%20raycasting%20start%20position))

(fn CastRayForwardfromComponentPosition
  (params (Component :type Scene%20Component%20Object%20Reference))
  (bind _returnvalue (Transformation|GetWorldLocation Component))
  (bind _outhit (Collision|LineTraceByChannel _returnvalue (+ _returnvalue (* (Math|Vector|GetForwardVector Component) 1000)) "TraceTypeQuery1" false 0 "None"))
  (return _outhit))

(fn GetInteractionComponents2
  (return (Variables|Interaction|GetInteractionComponents2)))