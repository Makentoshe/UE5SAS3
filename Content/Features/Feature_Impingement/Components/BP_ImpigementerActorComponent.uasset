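; Actor component that triggers an impingement scene on a target actor.
; It checks that the target implements the impingementable and elemental component-holder interfaces and fetches both components through interface messages.
; The scene is invoked on the impingementable component only if the elemental component reports at least one companioning elemental.
; Failed interface checks and empty elemental lists just print debug messages and skip the scene.
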(event EventBeginPlay)

(event EventTick
  (params (DeltaSeconds :type Float%20%28single-precision%29)))

(fn CauseImpingementforActor
  (params (ImpingementedActor :type Actor%20Object%20Reference))
  ;[1 1 1] Check is actor impingementable
  (if (Utilities|DoesObjectImplementInterface ImpingementedActor "/Game/Features/Feature_Impingement/Interfaces/BPI_ImpingementableActorComponentHolder.BPI_ImpingementableActorComponentHolder_C")
    (bind _component (Class|BPIImpingementableActorComponentHolder|GetIntercoursableActorComponent(Message) ImpingementedActor))
    (LocalVariables|SetImpingementableComponent _component)
    ;[1 1 1] Check actor may contain companion elementales
    (if (Utilities|DoesObjectImplementInterface ImpingementedActor "/Game/Features/Feature_Elemental/Interfaces/BPI_Elemental_ActorComponentHolder.BPI_Elemental_ActorComponentHolder_C")
      (bind _component_2 (Class|BPIElementalActorComponentHolder|GetElementalActorComponent(Message) ImpingementedActor))
      (LocalVariables|SetElementalComponent _component_2)
      (CallFunction|CauseImpingementforActorwithComponents (LocalVariables|GetImpingementableComponent) (LocalVariables|GetElementalComponent) ImpingementedActor)
      (else
        (Development|PrintString "Error: Doesn't implements elementales interface" true true "(R=1.000000,G=0.000000,B=0.032727,A=1.000000)")))
    (else
      (Development|PrintString "Error: Doesn't implements intercoursable interface" true true "(R=1.000000,G=0.000000,B=0.032727,A=1.000000)"))))

(fn CauseImpingementforActorwithComponents
  (params (ImpingementableComponent :type BP%20Impigementable%20Actor%20Component%20Object%20Reference) (ElementalComponent :type BP%20Actor%20Component%20Elemental%20Object%20Reference) (ImpingementActor :type Actor%20Object%20Reference))
  ;[1 1 1] Check impigment actor have an elementales
  (bind _newparam (Default|GetCompanioningElementals ElementalComponent))
  (if (< (Utilities|Array|Length _newparam) 1)
    (Development|PrintString "Skip intercourse - empty elementales" true true "(R=1.000000,G=0.107766,B=0.000000,A=1.000000)")
    (else
      (CallFunction|CauseImpingementScene ImpingementableComponent ElementalComponent ImpingementActor))))

(fn CauseImpingementScene
  (params (ImpingementableComponent :type BP%20Impigementable%20Actor%20Component%20Object%20Reference) (ElementalComponent :type BP%20Actor%20Component%20Elemental%20Object%20Reference) (ImpingementActor :type Actor%20Object%20Reference))
  (Default|InvokeImpigementScene ImpingementableComponent))