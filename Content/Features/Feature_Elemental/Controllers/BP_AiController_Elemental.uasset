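; AI controller for the elemental companion, which makes it follow the player character around.
; On possess it caches its pawn, the player and the player's elemental component, which serves as the follow point.
; Each tick it updates facing, then teleports the pawn to that point if too far away.
; Otherwise it moves the pawn toward the point at a distance-scaled speed and draws a debug line trace between them.
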(event EventPossess
  (params (PossessedPawn :type Pawn%20Object%20Reference))
  ;[1 1 1] Save controlled pawn to the global variable
  (Utilities|FlowControl|Sequence
    (:then_0
      (bind _asbp_elemental_character (Utilities|Casting|CastToBP_Elemental_Character PossessedPawn)
        (:then
          (Variables|Default|SetControlledCharacter _asbp_elemental_character))
        (:CastFailed
          (Development|PrintText "BP_AiControllerCharacterFollower - OnPossess - Cast ControlledCharacter issue" true true "(R=1.000000,G=0.000000,B=0.057610,A=1.000000)"))))
    (:then_1
      (bind _asbp_third_person_character (Utilities|Casting|CastToBP_ThirdPersonCharacter (Game|GetPlayerCharacter 0))
        (:then
          (bind _output_get (Variables|Default|SetPlayerCharacter _asbp_third_person_character))
          (bind _component (Default|GetElementalActorComponent _output_get))
          (Variables|Default|SetPlayerElementalComponent _component))
        (:CastFailed
          (Development|PrintText "BP_AiControllerCharacterFollower - OnPossess - Cast PlayerCharacter issue" true true "(R=1.000000,G=0.000000,B=0.057610,A=1.000000)"))))))

(event EventTick
  (params (DeltaSeconds :type Float%20%28single-precision%29))
  (bind _controlledcharacter (Variables|Default|GetControlledCharacter))
  (bind _controlledcharacter_2 (Variables|Default|GetControlledCharacter))
  (bind _playerelementalcomponent (Variables|Default|GetPlayerElementalComponent))
  (bind _returnvalue (Transformation|GetWorldLocation _playerelementalcomponent))
  (bind _returnvalue_2 (Transformation|GetActorLocation _controlledcharacter))
  (Variables|Default|SetDistanceFromControlledCharacterToPlayerCharacter (CallFunction|GetDistancetoPlayerCharacter))
  (Utilities|FlowControl|Sequence
    (:then_0
      ;[1 1 1] Be faced to the PlayerCharacter
      (if (> (Math|Vector|VectorLength (Transformation|GetVelocity (Variables|Default|GetControlledCharacter))) 1e+02)
        (bind _rotation (CallFunction|CalculateRotationActorVector _controlledcharacter_2 (Transformation|GetWorldLocation (Variables|Default|GetPlayerElementalComponent))))
        (else
          (CallFunction|CalculateRotationBetweenActors _controlledcharacter_2 (Variables|Default|GetPlayerCharacter))))
      (Transformation|SetActorRotation _controlledcharacter_2 _rotation))
    (:then_1
      ;[1 1 1] Teleport to player if too far
      (bind _wasteleported (CallFunction|TeleportAiControlledCharactertoPlayer))
      (if (not _wasteleported)
        ;[1 1 1] Move closer to PlayerCharacter when PlauerCharacter moves
        (Utilities|FlowControl|Sequence
          (:then_0
            (Default|MoveAiControlledCharacter (Variables|Default|GetControlledCharacter) (Math|Vector|Normalize (- _returnvalue _returnvalue_2)) (CallFunction|GetAiControlledCharacterSpeed 1e+01)))
          (:then_1
            (Collision|LineTraceByChannel _returnvalue _returnvalue_2 "TraceTypeQuery1" false 0 "ForOneFrame" true "(R=0.000000,G=0.188256,B=1.000000,A=1.000000)")))))))

(fn ConstructionScript)

(fn GetDistancetoPlayerCharacter
  (return (Transformation|GetDistanceTo (Variables|Default|GetControlledCharacter) (Variables|Default|GetPlayerCharacter))))

(fn MoveAiControlledCharacterCloser
  (bind _controlledcharacter (Variables|Default|GetControlledCharacter))
  (bind _returnvalue (Transformation|GetActorLocation _controlledcharacter))
  (bind _component (Default|GetElementalActorComponent (Variables|Default|GetPlayerCharacter)))
  (Utilities|FlowControl|Sequence
    (:then_0
      (Default|MoveAiControlledCharacter (Variables|Default|GetControlledCharacter) (Math|Vector|Normalize (- (Transformation|GetWorldLocation _component) _returnvalue)) (CallFunction|GetAiControlledCharacterSpeed 1e+01)))
    (:then_1
      (Collision|LineTraceByChannel (Transformation|GetWorldLocation _component) _returnvalue "TraceTypeQuery1" false 0 "ForOneFrame" true "(R=0.000000,G=0.188256,B=1.000000,A=1.000000)"))))

(fn GetAiControlledCharacterSpeed
  (params (Multiplier :type Float%20%28double-precision%29))
  (return (* Multiplier (/ (- (Variables|Default|GetDistanceFromControlledCharacterToPlayerCharacter) (Variables|Const|GetFurtherDistance)) (Variables|/Script/Engine.CharacterMovementComponent|GetMaxFlySpeed (Variables|/Script/Engine.Character|GetCharacterMovement (Variables|Default|GetControlledCharacter)))))))

(fn TeleportAiControlledCharactertoPlayer
  (if (> (Variables|Default|GetDistanceFromControlledCharacterToPlayerCharacter) (Variables|Const|GetTeleportDistance))
    (bind _component (Default|GetElementalActorComponent (Variables|Default|GetPlayerCharacter)))
    (bind _returnvalue (Transformation|Teleport (Variables|Default|GetControlledCharacter) (Transformation|GetWorldLocation _component) "0, 0, 0"))
    (return _returnvalue)
    (else
      (return false))))