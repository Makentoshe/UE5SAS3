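; AI controller that makes a possessed elemental character follow and face the player.
; Each tick it keeps the pawn within a distance band, approaching an offset shoulder point or backing away, with speed scaled by distance.
; Retreat adds a sideways strafe chosen by a dot product of pawn and player axes.
; A custom hit event uses a similar dot test to sidestep with debug prints.
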(event Custom|CustomEventHit
  (params (Hit%20Target :type Actor%20Object%20Reference) (Hit :type Hit%20Result%20Structure))
  (bind _controlledcharacter (Variables|Default|GetControlledCharacter))
  (bind _controlledcharacter_2 (Variables|Default|GetControlledCharacter))
  (bind _returnvalue (Transformation|GetActorRightVector _controlledcharacter))
  ;[1 1 1] Move around character
  (if (< (Math|Vector|DotProduct (Transformation|GetActorForwardVector Hit%20Target) (Transformation|GetActorRightVector (.HitActor (Collision|BreakHitResult Hit)))) 0.0)
    (Development|PrintString "Move pawn to right")
    (Default|MoveControlledCharacter _controlledcharacter_2 _returnvalue 1e+03)
    (else
      (Development|PrintString "Move pawn to left")
      (Default|MoveControlledCharacter _controlledcharacter_2 (Math|Vector|RotateVector _returnvalue "0,180.000000,0.000000") 1e+03))))

(event EventPossess
  (params (PossessedPawn :type Pawn%20Object%20Reference))
  ;[1 1 1] Save controlled pawn to the global variable
  (bind _asbp_elemental_character (Utilities|Casting|CastToBP_Elemental_Character PossessedPawn)
    (:then
      (Variables|Default|SetControlledCharacter _asbp_elemental_character))
    (:CastFailed
      (Development|PrintText "BP_AiControllerCharacterFollower - OnPossess - Cast issue" true true "(R=1.000000,G=0.000000,B=0.057610,A=1.000000)"))))

(event EventTick
  (params (DeltaSeconds :type Float%20%28single-precision%29))
  (bind _controlledcharacter (Variables|Default|GetControlledCharacter))
  (bind _returnvalue (Transformation|GetActorRightVector _controlledcharacter))
  ;[0.7387 0 1] Player character following
  ;;[1 1 1] Get Distance to the Player Character
  (Variables|Default|SetDistanceToCharacter (Transformation|GetDistanceTo (Variables|Default|GetControlledCharacter) (Game|GetPlayerCharacter 0)))
  ;;[1 1 1] Always be faced to the character
  (CallFunction|FaceTargettotheActor (Variables|Default|GetControlledCharacter) (Game|GetPlayerCharacter 0))
  ;;[1 1 1] Calculate pawn position near the player character
  (Utilities|CalculatePawnPosition
    (:Should%20be%20closer
      ;;[1 1 1] Move pawn closer to the player character
      (Default|MoveControlledCharacter (Variables|Default|GetControlledCharacter) (Utilities|GetMoveDirectionVector) (Utilities|GetConvergenceSpeedScale)))
    (:Should%20be%20further
      ;;[1 1 1] Get a pawn strafe vector
      (if (< (Math|Vector|DotProduct (Transformation|GetActorForwardVector (Variables|Default|GetControlledCharacter)) (Transformation|GetActorRightVector (Game|GetPlayerCharacter 0))) 0.0)
        (Variables|Default|SetDivergenceStrafeVector _returnvalue)
        (else
          (Variables|Default|SetDivergenceStrafeVector (Math|Vector|RotateVector _returnvalue "0,180.000000, 0"))))
      ;;[1 1 1] Move pawn further from the player character
      (Default|MoveControlledCharacter (Variables|Default|GetControlledCharacter) (+ (Math|Vector|RotateVector (Utilities|GetMoveDirectionVector) "0,180.000000,0.000000") (Variables|Default|GetDivergenceStrafeVector)) (Utilities|GetDivergenceSpeedScale)))))

(fn ConstructionScript)

(fn FaceTargettotheActor
  (params (Target :type Actor%20Object%20Reference) (Actor :type Actor%20Object%20Reference))
  ;[1 1 1] Always be faced to the character
  (bind _rotation (CallFunction|CalculateRotationBetweenActors Target Actor))
  (Transformation|SetActorRotation Target _rotation))