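; Actor component that manages a capped list of companion elementals, one of which follows in the world.
; Adding an elemental stores it and fires an event; the first one added is spawned at once and recorded as the following elemental.
; Spawning creates the creature from the wrapper's class with collision disabled, assigns the elemental AI controller, then fires a spawn event.
; Getters expose the list and current follower.
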(fn AddCompanioningElemental
  (params (CreatureElementalWrapper :type BP%20Elemental%20Creature%20Wrapper%20Object%20Reference))
  (bind _companioningelementals (Variables|Default|GetCompanioningElementals))
  ;[1 1 1] Is able to contain more elementales
  (if (< (Utilities|Array|Length (Variables|Default|GetCompanioningElementals)) (Variables|Settings|GetMaxElementalesCount))
    ;[1 1 1] Add elemental to the list
    (Utilities|Array|Add _companioningelementals CreatureElementalWrapper)
    (Default|CallOnAddCompanionElemental _companioningelementals)
    ;[1 1 1] Is able to spawn follower immediately
    (if (== (Utilities|Array|Length (Variables|Default|GetCompanioningElementals)) 1)
      (CallFunction|SpawnCompanioningElemental CreatureElementalWrapper)
      (Variables|Default|SetFollowingElemental CreatureElementalWrapper))
    (else
      (Development|PrintString "Elementals list full"))))

(fn SpawnCompanioningElemental
  (params (ElementalCreatureWrapper :type BP%20Elemental%20Creature%20Wrapper%20Object%20Reference))
  (bind _returnvalue (Game|SpawnActorfromClass (Utilities|Struct|BreakElementalCreatureStructure (Variables|/Game/Features/Feature_Elemental/Structures/Wrappers/BP_ElementalCreatureWrapper.BP_ElementalCreatureWrapper_C|GetElementalCreatureStructure ElementalCreatureWrapper)) (Math|Transform|MakeTransform (Transformation|GetWorldLocation) "0, 0, 0" (Math|Conversions|ToVector(Float) (LocalVariables|GetScale))) "AlwaysSpawn" 0 0))
  (Collision|SetActorEnableCollision _returnvalue false)
  (Variables|/Script/Engine.Pawn|SetAIControllerClass _returnvalue "/Game/Features/Feature_Elemental/Controllers/BP_AiController_Elemental.BP_AiController_Elemental_C")
  (Pawn|SpawnDefaultController _returnvalue)
  (Default|CallOnSpawnCompanionElemental _returnvalue))

(fn GetCompanioningElementals
  (return (Variables|Default|GetCompanioningElementals)))

(fn GetFollowingElemental
  (return (Variables|Default|GetFollowingElemental)))