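; Inventory UI actor component that shows and hides the character inventory widget for its owning player controller.
; On BeginPlay it binds handlers to its show and hide inventory events.
; Showing creates WBP_CharacterInventory, fills it with item and companion elemental entries, then enables game-and-UI input with the cursor.
; Hiding removes and clears the widget, then restores game-only input without the cursor.
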(event Custom|OnShowInventoryWidgetBp_Event
  (params (InventoryItems :type Array%20of%20Inventory%20Item%20Structure%20Wrapper%20Object%20References) (CompanionElementales :type Array%20of%20BP%20Elemental%20Creature%20Wrapper%20Object%20References))
  ;[1 1 1] Showing inventory
  ;;[1 1 1] Create inventory widget
  (bind _returnvalue (UserInterface|CreateWidget "/Game/Features/Feature_Inventory/Widgets/WBP_CharacterInventory.WBP_CharacterInventory_C" (Variables|Default|GetOwnerController)))
  (bind _output_get (Variables|UserInterface|SetInventoryWidget _returnvalue))
  ;;[1 1 1] Fill inventory widget with items
  (Default|UpdateInventoryEntries _output_get InventoryItems)
  (Default|UpdateCompanionEntries _output_get CompanionElementales)
  ;;[1 1 1] Get controll from the player
  (Input|SetInputModeGameandUI (Variables|Default|GetOwnerController) (Variables|UserInterface|GetInventoryWidget) "DoNotLock" true)
  (UserInterface|Viewport|AddtoViewport (Variables|UserInterface|GetInventoryWidget) 0)
  (Variables|/Script/Engine.PlayerController|SetbShowMouseCursor (Variables|Default|GetOwnerController) true))

(event Custom|OnHideInventoryWidgetEvent
  (bind _ownercontroller (Variables|Default|GetOwnerController))
  ;[1 1 1] Hiding inventory
  ;;[1 1 1] Remove inventory widget
  (Widget|RemovefromParent (Variables|UserInterface|GetInventoryWidget))
  (Variables|UserInterface|SetInventoryWidget 0)
  ;;[1 1 1] Return controll to the player
  (Input|SetInputModeGameOnly _ownercontroller)
  (Variables|/Script/Engine.PlayerController|SetbShowMouseCursor _ownercontroller false))

(event EventBeginPlay
  ;[1 1 1] Showing inventory
  (EventDispatchers|BindEventtoOnShowInventoryWidgetBp (delegate Custom|OnShowInventoryWidgetBp_Event))
  ;[1 1 1] Hiding inventory
  (EventDispatchers|AssignOnHideInventoryWidget (delegate Custom|OnHideInventoryWidgetEvent)))