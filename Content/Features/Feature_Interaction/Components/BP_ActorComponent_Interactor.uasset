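; Actor component that tracks nearby interactions, cycles a wrapping selection through them and executes the selected one.
; Add and remove events maintain a list of spawned wrapper actors around each interaction structure, looked up by structure equality, and notify InteractorUiActorComponent.
; Interacting dispatches by type: inventory items go to InventoryActorComponent and are destroyed, while environment actors receive an interaction event.
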(event Custom|OnNearbyInteractionEvent
  ;[1 1 1] Player somehow interacts with this item
  (if (!= (Utilities|Array|Length (Variables|Default|GetNearbyInteractionWrappers)) 0) ; If not empty interactions
    (if (> (Utilities|Array|Length (Variables|Default|GetNearbyInteractionWrappers)) (Variables|Default|GetSelectedInteractionIndex)) ; If selection value valid
      (CallFunction|InternalonNearbyInteraction (Utilities|Array|Get(acopy) (Variables|Default|GetNearbyInteractionWrappers) (Variables|Default|GetSelectedInteractionIndex)))
      (else
        (Development|PrintString "Error: Issue with NearbyInteractions list and selection" true true "(R=1.000000,G=0.000000,B=0.026892,A=1.000000)")))
    (else
      (Development|PrintString "Error: NearbyInteractionsWidget isn't visible - cant interact with the items" true true "(R=1.000000,G=0.000000,B=0.026892,A=1.000000)"))))

(event Custom|OnAddNearbyInteractionEvent
  (params (Structure :type Nearby%20Interaction%20Structure%20Structure))
  ;[1 1 1] Add NearbyInteraction structure to the map
  (bind _wrapped (Utilities|Wrap Structure)
    (:%20%20
      (Utilities|Array|Add (Variables|Default|GetNearbyInteractionWrappers) _wrapped)
      (Default|CallOnAddNearbyInteraction (Variables|Default|GetInteractorUiActorComponent) _wrapped))))

(event Custom|OnRemoveNearbyInteractionEvent
  (params (Structure :type Nearby%20Interaction%20Structure%20Structure))
  ;[1 1 1] Remove NearbyInteractionStructure from the map
  (bind (_wrapper __) (CallFunction|FindWrapper (Variables|Default|GetNearbyInteractionWrappers) Structure))
  (if __ ; Is map contains the item
    (Default|CallOnRemoveNearbyInteraction (Variables|Default|GetInteractorUiActorComponent) _wrapper)
    (bind _returnvalue (Utilities|Array|RemoveItem (Variables|Default|GetNearbyInteractionWrappers) _wrapper))
    (if _returnvalue ; If item was removed
      (bind _output_get (Variables|Default|SetSelectedInteractionIndex (Math|Integer|Max(Integer) (Math|Integer|Min(Integer) (Utilities|Array|LastIndex (Variables|Default|GetNearbyInteractionWrappers)) (Variables|Default|GetSelectedInteractionIndex)))))
      (Default|CallOnChangeSelectedNearbyInteractionIndex (Variables|Default|GetInteractorUiActorComponent) _output_get)
      (else
        (Development|PrintString "Error: Cant remove NearbyInteractionsWrapper from the map" true true "(R=1.000000,G=0.000000,B=0.070807,A=1.000000)")))
    (else
      (Development|PrintString "Error: Cant find NearbyInteractionsWrapper in the map" true true "(R=1.000000,G=0.000000,B=0.070807,A=1.000000)"))))

(event Custom|OnNextSelectedNearbyInteractionIndexEvent
  ;[1 1 1] On Next item selection event
  (if (< (+ (Variables|Default|GetSelectedInteractionIndex) 1) (Utilities|Array|Length (Variables|Default|GetNearbyInteractionWrappers)))
    (Variables|Default|SetSelectedInteractionIndex (+ (Variables|Default|GetSelectedInteractionIndex) 1))
    (else
      (Variables|Default|SetSelectedInteractionIndex 0)))
  (Default|CallOnChangeSelectedNearbyInteractionIndex (Variables|Default|GetInteractorUiActorComponent) (Variables|Default|GetSelectedInteractionIndex)))

(event Custom|OnPrevSelectedNearbyInteractionIndexEvent
  ;[1 1 1] On Previous item selection event
  (if (< (- (Variables|Default|GetSelectedInteractionIndex) 1) 0)
    (Variables|Default|SetSelectedInteractionIndex (Math|Integer|Max(Integer) (Utilities|Array|LastIndex (Variables|Default|GetNearbyInteractionWrappers))))
    (else
      (Variables|Default|SetSelectedInteractionIndex (- (Variables|Default|GetSelectedInteractionIndex) 1))))
  (Default|CallOnChangeSelectedNearbyInteractionIndex (Variables|Default|GetInteractorUiActorComponent) (Variables|Default|GetSelectedInteractionIndex)))

(event EventEndPlay
  (params (EndPlayReason :type EEndPlayReason%20Enum :default "Destroyed"))
  ;[1 1 1] Releasse
  (Utilities|Array|Clear (Variables|Default|GetNearbyInteractionWrappers)))

(event EventBeginPlay
  (Utilities|FlowControl|Sequence
    (:then_0
      ;[1 1 1] Add NearbyInteraction structure to the map
      (EventDispatchers|BindEventtoOnAddNearbyInteraction (delegate Custom|OnAddNearbyInteractionEvent))
      ;[1 1 1] Remove NearbyInteractionStructure from the map
      (EventDispatchers|AssignOnRemoveNearbyInteraction (delegate Custom|OnRemoveNearbyInteractionEvent)))
    (:then_1
      ;[1 1 1] On Next item selection event
      (EventDispatchers|AssignOnNextSelectedNearbyInteractionIndex (delegate Custom|OnNextSelectedNearbyInteractionIndexEvent))
      ;[1 1 1] On Previous item selection event
      (EventDispatchers|AssignOnPrevSelectedNearbyInteractionIndex (delegate Custom|OnPrevSelectedNearbyInteractionIndexEvent)))
    (:then_2
      ;[1 1 1] Player somehow interacts with this item
      (EventDispatchers|AssignOnNearbyInteraction (delegate Custom|OnNearbyInteractionEvent)))))

(fn InternalonNearbyInteraction
  (params (NearbyInteractionWrapper :type Nearby%20Interaction%20Wrapper%20Object%20Reference))
  (LocalVariables|SetNearbyInteractionStructure (Variables|/Script/Sas3.NearbyInteractionWrapper|GetNearbyInteractionStructure NearbyInteractionWrapper))
  (switch Utilities|FlowControl|Switch|SwitchonNearbyInteractionType (.NearbyInteractionType (Utilities|Struct|BreakNearbyInteractionStructure (Variables|/Script/Sas3.NearbyInteractionWrapper|GetNearbyInteractionStructure NearbyInteractionWrapper)))
    (:None
      (Development|PrintString "Error: NearbyAction type is None" true true "(R=1.000000,G=0.010790,B=0.000000,A=1.000000)" :!pinned true) ; None: shouldn't be reachable
    )
    (:Inventory
      ;[1 1 1] Inventory interaction
      (bind _asinventory_item_actor (Utilities|Casting|CastToInventoryItemActor (.Actor (Utilities|Struct|BreakNearbyInteractionStructure (Variables|/Script/Sas3.NearbyInteractionWrapper|GetNearbyInteractionStructure NearbyInteractionWrapper))))
        (:then
          (CallFunction|InternalonInventoryInteraction _asinventory_item_actor (LocalVariables|GetNearbyInteractionStructure)))
        (:CastFailed
          (Development|PrintString "Error: Cant cast object to InventoryItemActor" true true "(R=1.000000,G=0.000000,B=0.041855,A=1.000000)"))))
    (:Environment
      ;[1 1 1] Environment interaction
      (bind _asbp_environment_item_actor (Utilities|Casting|CastToBP_EnvironmentItemActor (.Actor (Utilities|Struct|BreakNearbyInteractionStructure (Variables|/Script/Sas3.NearbyInteractionWrapper|GetNearbyInteractionStructure NearbyInteractionWrapper))))
        (:then
          (CallFunction|InternalonEnvironmentInteraction _asbp_environment_item_actor))
        (:CastFailed
          (Development|PrintString "Error: Cant cast object toEnvironmentItemActor" true true "(R=1.000000,G=0.938499,B=0.000000,A=1.000000)"))))))

(fn InternalonInventoryInteraction
  (params (InventoryItemActor :type Inventory%20Item%20Actor%20Object%20Reference) (Structure :type Nearby%20Interaction%20Structure%20Structure))
  (bind _inventorymeta (Variables|/Script/Sas3.InventoryItemActor|GetInventoryMeta InventoryItemActor))
  (bind (_itemcount _stacksize) (Utilities|Struct|BreakInventoryMetaStructure _inventorymeta))
  (Utilities|FlowControl|Sequence
    (:then_0
      ;[1 1 1] Add item to the inventory
      (Class|InventoryActorComponent|AddInventoryItem (Variables|Default|GetInventoryActorComponent) (Utilities|Struct|MakeInventoryItemStructure _itemcount _stacksize (Utilities|Struct|BreakGameItemStructure (Variables|/Script/Sas3.GameItemActor|GetGameItem InventoryItemActor)))))
    (:then_1
      (Actor|DestroyActor InventoryItemActor :!pinned true) ; Destroying will cause OnEndOverlap which cause widget update
      (CallFunction|OnRemoveNearbyInteractionEvent Structure))
    (:then_2
      ;[1 1 1] Decrease index if it out of the length bound
      (bind _output_get (Variables|Default|SetSelectedInteractionIndex (Math|Integer|Max(Integer) (Math|Integer|Min(Integer) (Utilities|Array|LastIndex (Variables|Default|GetNearbyInteractionWrappers)) (Variables|Default|GetSelectedInteractionIndex)))))
      (Default|CallOnChangeSelectedNearbyInteractionIndex (Variables|Default|GetInteractorUiActorComponent) _output_get))))

(fn InternalonEnvironmentInteraction
  (params (EnvironmentItemActor :type BP%20Environment%20Item%20Actor%20Object%20Reference))
  (Default|OnEnvironmentNearbyInteractionEvent EnvironmentItemActor))

(fn FindWrapper
  (params (Array :type Array%20of%20Nearby%20Interaction%20Wrapper%20Object%20References) (NearbyInteractionStructure :type Nearby%20Interaction%20Structure%20Structure))
  (for _array_element Array
    (bind __ (CallFunction|Equals (Variables|/Script/Sas3.NearbyInteractionWrapper|GetNearbyInteractionStructure _array_element) NearbyInteractionStructure))
    (if __
      (return _array_element __)))
  (return 0 false))