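; Actor component that manages a character's HUD for obtained inventory items and nearby interactions.
; On BeginPlay it creates both widgets for the owner controller, keeping the obtainings widget hidden in the viewport.
; Adding an item shows that widget, and a list entry-release callback hides it once empty.
; Functions forward interaction additions, removals and selection changes to the interaction widget, adding it to the viewport when needed and removing it when empty.
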(event Custom|OnEachObtainedItemRemoveEvent
  (params (Widget :type User%20Widget%20Object%20Reference))
  ;[1 1 1] Obtainings - callback for hiding widget if it is empty after removeing entry
  (if (< (Class|ListView|GetNumItems (Variables|/Game/Features/Feature_CharacterHud/Widgets/WBP_CharacterObtainer.WBP_CharacterObtainer_C|GetObtainingsContainer (Variables|Default|GetObtainingsWidget))) 1)
    (Widget|SetVisibility (Variables|Default|GetObtainingsWidget) "Hidden")))

(event EventBeginPlay
  (Utilities|FlowControl|Sequence
    (:then_0
      (Utilities|FlowControl|Sequence
        (:then_0
          ;[1 1 1] Obtainings - initialize widget
          (bind _returnvalue (UserInterface|CreateWidget "/Game/Features/Feature_CharacterHud/Widgets/WBP_CharacterObtainer.WBP_CharacterObtainer_C" (Variables|Default|GetOwnerController)))
          (bind _output_get (Variables|Default|SetObtainingsWidget _returnvalue))
          (Widget|SetVisibility _output_get "Hidden")
          (UserInterface|Viewport|AddtoViewport _output_get 0))
        (:then_1
          ;[1 1 1] Obtainings - callback for hiding widget if it is empty after removeing entry
          (EventDispatchers|AssignBPonEntryReleased (Variables|/Game/Features/Feature_CharacterHud/Widgets/WBP_CharacterObtainer.WBP_CharacterObtainer_C|GetObtainingsContainer (Variables|Default|GetObtainingsWidget)) (delegate Custom|OnEachObtainedItemRemoveEvent)))))
    (:then_1
      (Utilities|FlowControl|Sequence
        (:then_0
          ;[1 1 1] NearbyInteractions - Initialize widget
          (bind _returnvalue_2 (UserInterface|CreateWidget "/Game/Features/Feature_Interaction/Widgets/WBP_CharacterInteraction.WBP_CharacterInteraction_C" (Variables|Default|GetOwnerController)))
          (Variables|Default|SetNearbyInteractionsWidget _returnvalue_2))))))

(event EventTick
  (params (DeltaSeconds :type Float%20%28single-precision%29)))

(fn AddObtainedInventoryItem
  (params (InventoryItemWrapper :type Inventory%20Item%20Structure%20Wrapper%20Object%20Reference))
  (Class|ListView|AddItem (Variables|/Game/Features/Feature_CharacterHud/Widgets/WBP_CharacterObtainer.WBP_CharacterObtainer_C|GetObtainingsContainer (Variables|Default|GetObtainingsWidget)) InventoryItemWrapper)
  (Widget|SetVisibility (Variables|Default|GetObtainingsWidget) "Visible"))

(fn AddNearbyInteraction
  (params (NearbyInteractionWrapper :type Nearby%20Interaction%20Wrapper%20Object%20Reference))
  (bind _nearbyinteractionswidget (Variables|Default|GetNearbyInteractionsWidget))
  (Default|OnAddNearbyInteractionEntryEvent _nearbyinteractionswidget NearbyInteractionWrapper)
  (if (not (Widget|IsVisible _nearbyinteractionswidget))
    (UserInterface|Viewport|AddtoViewport _nearbyinteractionswidget 0)))

(fn RemoveNearbyInteraction
  (params (NearbyInteractionWrapper :type Nearby%20Interaction%20Wrapper%20Object%20Reference))
  (bind _nearbyinteractionswidget (Variables|Default|GetNearbyInteractionsWidget))
  (Default|OnRemoveNearbyInteractionEntryEvent _nearbyinteractionswidget NearbyInteractionWrapper)
  (if (not (> (Class|ListView|GetNumItems (Variables|/Game/Features/Feature_Interaction/Widgets/WBP_CharacterInteraction.WBP_CharacterInteraction_C|GetInteractionActionsContainer _nearbyinteractionswidget)) 0))
    (Widget|RemovefromParent _nearbyinteractionswidget)))

(fn ChangeNearbyInteractionSelection
  (params (NewIndex :type Integer))
  (Default|OnNearbyInteractionSelectionChangedEvent (Variables|Default|GetNearbyInteractionsWidget) NewIndex))