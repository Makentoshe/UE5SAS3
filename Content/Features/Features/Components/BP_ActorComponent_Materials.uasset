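; Actor component that creates and holds dynamic material instances for its owner's meshes to drive a disperse effect.
; InitializeDynamicMaterials wraps every material slot of a given mesh component in a dynamic instance and appends it to a shared array without clearing it.
; SetDisperseColor and SetDisperseValue write a vector or scalar parameter, named by variables, to all cached instances at once.
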(fn SetDisperseColor
  (params (Color :type Linear%20Color%20Structure%20%28by%20ref%29))
  (for _array_element (CallFunction|GetDynamicMaterials)
    (Rendering|Material|SetVectorParameterValue _array_element (Variables|Names|Disperse|GetDisperseColorName) Color :!class /Script/Engine.MaterialInstanceDynamic)))

(fn SetDisperseValue
  (params (Value :type Float%20%28double-precision%29%20%28by%20ref%29))
  (for _array_element (CallFunction|GetDynamicMaterials)
    (Rendering|Material|SetScalarParameterValue _array_element (Variables|Names|Disperse|GetDisperseValueName) Value :!class /Script/Engine.MaterialInstanceDynamic)))

(fn GetDynamicMaterials
  (return (Variables|Default|GetDynamicMaterialInstances)))

(fn InitializeDynamicMaterials
  (params (MeshComponent :type Mesh%20Component%20Object%20Reference))
  (for (_array_element _array_index) (Rendering|Material|GetMaterials MeshComponent)
    (bind _returnvalue (Rendering|Material|CreateDynamicMaterialInstance MeshComponent _array_index _array_element "None" :!class /Script/Engine.PrimitiveComponent))
    (Utilities|Array|Add (Variables|Default|GetDynamicMaterialInstances) _returnvalue)))