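; Actor component that manages the on-screen widget listing items the character obtains.
; On BeginPlay it creates a hidden WBP_CharacterObtainer for player 0 and adds it to the viewport.
; Its OnAddObtainedItem event feeds each item wrapper into the ObtainingsContainer and shows the widget.
; The container's entry-released callback hides the widget once no items remain.
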(event Custom|OnEachObtainedItemRemoveEvent
  (params (Widget :type User%20Widget%20Object%20Reference))
  ;[1 1 1] Implement Removing InventoryItem from the obtainings widget
  (if (< (Class|ListView|GetNumItems (Variables|/Game/Features/Feature_Ui_Obtained/Widgets/WBP_CharacterObtainer.WBP_CharacterObtainer_C|GetObtainingsContainer (Variables|Default|GetObtainingsWidget))) 1)
    (Widget|SetVisibility (Variables|Default|GetObtainingsWidget) "Hidden")))

(event Custom|OnEachObtainedItemAddEvent
  (params (Wrapper :type Inventory%20Item%20Structure%20Wrapper%20Object%20Reference))
  ;[1 1 1] Implement Adding InventoryItem to the obtainings widget
  (Class|ListView|AddItem (Variables|/Game/Features/Feature_Ui_Obtained/Widgets/WBP_CharacterObtainer.WBP_CharacterObtainer_C|GetObtainingsContainer (Variables|Default|GetObtainingsWidget)) Wrapper)
  (Widget|SetVisibility (Variables|Default|GetObtainingsWidget) "Visible"))

(event EventBeginPlay
  (Utilities|FlowControl|Sequence
    (:then_0
      ;[1 1 1] Initialize Obtainings widget
      (bind _returnvalue (UserInterface|CreateWidget "/Game/Features/Feature_Ui_Obtained/Widgets/WBP_CharacterObtainer.WBP_CharacterObtainer_C" (Game|GetPlayerController 0)))
      (bind _output_get (Variables|Default|SetObtainingsWidget _returnvalue))
      (Widget|SetVisibility _output_get "Hidden")
      (UserInterface|Viewport|AddtoViewport _output_get 0))
    (:then_2
      ;[1 1 1] Implement Adding InventoryItem to the obtainings widget
      (EventDispatchers|AssignOnAddObtainedItem (delegate Custom|OnEachObtainedItemAddEvent))
      ;[1 1 1] Implement Removing InventoryItem from the obtainings widget
      (EventDispatchers|AssignBPonEntryReleased (Variables|/Game/Features/Feature_Ui_Obtained/Widgets/WBP_CharacterObtainer.WBP_CharacterObtainer_C|GetObtainingsContainer (Variables|Default|GetObtainingsWidget)) (delegate Custom|OnEachObtainedItemRemoveEvent)))))