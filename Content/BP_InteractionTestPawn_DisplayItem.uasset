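; BP_InteractionTestPawn_DisplayItem is a test pawn for the interaction system that shows item information when selected.
; Selection events from its interaction component make the display component show a widget with a hardcoded name and description.
; Unselected and unavailable events both hide that widget.
; It also exposes its interaction component through a getter and includes a helper that fetches an actor's interactor component via interface.
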(event OnInteractionComponentSelectedDelegate(BP_InteractionComponent)
  (Default|ShowDisplayWidget (Variables|Default|GetBP_DisplayComponent) (Utilities|Struct|MakeSDisplayItem "Test Item" "A short item description just in few words")))

(event OnInteractionComponentUnselectedDelegate(BP_InteractionComponent)
  (Default|HideDisplayWidget (Variables|Default|GetBP_DisplayComponent)))

(event OnInteractionComponentUnavailableDelegate(BP_InteractionComponent)
  (Default|HideDisplayWidget (Variables|Default|GetBP_DisplayComponent)))

(fn ConstructionScript)

(fn GetInteractionComponent
  (return (Variables|Default|GetBP_InteractionComponent)))