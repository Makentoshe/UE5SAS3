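; Actor component that keeps a list of nearby interaction actions for its owner, apparently a prototype interactor.
; On BeginPlay it gets the owner's InteractorUi component through a holder interface, printing an error if the interface is missing.
; Adding or removing an action updates the NearbyActions list and notifies that UI component.
; A Z key debug hook prints each nearby action's index, title and type.
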(event EventBeginPlay
  (bind _returnvalue (Components|GetOwner))
  ;[1 1 1] Define InteractorUiActorComponent
  (if (Utilities|DoesObjectImplementInterface _returnvalue "/Game/Prototype/ActorComponents/BPI_ActorComponent_InteractorUi_Holder.BPI_ActorComponent_InteractorUi_Holder_C")
    (bind _interactoruicomponent (Class|BPIActorComponentInteractorUiHolder|GetInteractorUiActorComponent(Message) _returnvalue))
    (Variables|Default|SetInteractorUiActorComponent _interactoruicomponent)
    (else
      (Development|PrintString "Error: Owner doesn't implements   interface" true true "(R=1.000000,G=0.000000,B=0.093436,A=1.000000)"))))

(event Input|KeyboardEvents|Z
  (params (Key :type Key%20Structure :default "None"))
  (:Pressed
    (for (_array_element _array_index) (Variables|Default|GetNearbyActions)
      (Development|PrintString (Utilities|String|Append (Utilities|String|ToString(Integer) _array_index) (Utilities|String|ToString(Name) (.ActionTitle (Utilities|Struct|BreakNearbyActionStructure _array_element))) "(type=" (Utilities|String|EnumtoString (.ActionType (Utilities|Struct|BreakNearbyActionStructure _array_element))) ")")))))

(fn AddtoActionList
  (params (NearbyAction :type Nearby%20Action%20Structure%20Structure))
  (Utilities|Array|Add (Variables|Default|GetNearbyActions) NearbyAction)
  (Default|OnAddNearbyActionEvent (Variables|Default|GetInteractorUiActorComponent) NearbyAction))

(fn RemovefromActionList
  (params (NearbyAction :type Nearby%20Action%20Structure%20Structure))
  (Utilities|Array|RemoveItem (Variables|Default|GetNearbyActions) NearbyAction)
  (Default|OnRemoveNearbyActionEvent (Variables|Default|GetInteractorUiActorComponent) NearbyAction))