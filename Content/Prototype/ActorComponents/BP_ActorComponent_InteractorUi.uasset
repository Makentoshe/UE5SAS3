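; Actor component that drives the nearby-actions UI for an interactor, showing, scrolling and executing interaction options.
; On BeginPlay it creates the WBP_NearbyActions widget and gets the owner's Interactor and Inventory components through interfaces.
; Add and remove events toggle the widget in the viewport, while scroll events write the selected index back to the Interactor.
; Interacting adds inventory items and destroys their actor; environment actions only print.
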(event Custom|OnAddNearbyActionEvent
  (params (NearbyAction :type Nearby%20Action%20Structure%20Structure))
  (bind _nearbyactionswidget (Variables|Default|GetNearbyActionsWidget))
  ;[1 1 1] Adding NearbyAction to the UI
  (Default|AddNearbyActionasChildWidget _nearbyactionswidget NearbyAction)
  (if (not (Widget|IsVisible _nearbyactionswidget))
    (UserInterface|Viewport|AddtoViewport _nearbyactionswidget 0)))

(event Custom|OnRemoveNearbyActionEvent
  (params (NearbyAction :type Nearby%20Action%20Structure%20Structure))
  (bind _nearbyactionswidget (Variables|Default|GetNearbyActionsWidget))
  ;[1 1 1] Removing NearbyAction from the UI
  (Default|RemoveNearbyActionfromChildWidget _nearbyactionswidget NearbyAction)
  (if (not (Class|PanelWidget|HasAnyChildren (Variables|/Game/Widgets/WBP_NearbyActions.WBP_NearbyActions_C|GetNearbyActionsContainer _nearbyactionswidget)))
    (Widget|RemovefromParent (Variables|Default|GetNearbyActionsWidget))))

(event Custom|OnNextSelectedNearbyActionIndexEvent
  ;[1 1 1] NearbyAction selection scrolling
  (bind _selection (Default|NextSelectedNearbyActionIndex (Variables|Default|GetNearbyActionsWidget)))
  (Variables|/Game/Prototype/ActorComponents/BP_ActorComponent_Interactor.BP_ActorComponent_Interactor_C|SetNearbyActionSelection (Variables|Default|GetInteractorActorComponent) _selection))

(event Custom|OnPrevSelectedNearbyActionIndexEvent
  ;[1 1 1] NearbyAction selection scrolling
  (bind _selection (Default|PrevSelectedNearbyActionIndex (Variables|Default|GetNearbyActionsWidget)))
  (Variables|/Game/Prototype/ActorComponents/BP_ActorComponent_Interactor.BP_ActorComponent_Interactor_C|SetNearbyActionSelection (Variables|Default|GetInteractorActorComponent) _selection))

(event Custom|OnNearbyActionInteractionEvent
  (params (NearbyActionSelectedIndex :type Integer))
  ;[1 1 1] Get selected NearbyAction widget
  (if (Widget|IsVisible (Variables|Default|GetNearbyActionsWidget))
    (bind _aswbp_nearby_actions_element (Utilities|Casting|CastToWBP_NearbyActions_Element (Class|PanelWidget|GetChildat (Variables|/Game/Widgets/WBP_NearbyActions.WBP_NearbyActions_C|GetNearbyActionsContainer (Variables|Default|GetNearbyActionsWidget)) NearbyActionSelectedIndex)))
    ;[1 1 1] Get NearbyAction type
    (switch Utilities|FlowControl|Switch|SwitchonENearbyActionType (.ActionType (Utilities|Struct|BreakNearbyActionStructure (Variables|/Game/Widgets/WBP_NearbyActions_Element.WBP_NearbyActions_Element_C|GetNearbyAction _aswbp_nearby_actions_element)))
      (:None
        (Development|PrintString "Error: NearbyAction type is None" true true "(R=1.000000,G=0.010790,B=0.000000,A=1.000000)" :!pinned true) ; None: shouldn't be reachable
      )
      (:Inventory
        ;[1 1 1] Add item to the Inventory and destroy the actor
        (Class|InventoryActorComponent|AddInventoryItem (Variables|Default|GetInventoryActorComponent) (.InventoryItem (Utilities|Struct|BreakNearbyActionStructure (Variables|/Game/Widgets/WBP_NearbyActions_Element.WBP_NearbyActions_Element_C|GetNearbyAction _aswbp_nearby_actions_element))))
        (Actor|DestroyActor (.NearbyActionActor (Utilities|Struct|BreakNearbyActionStructure (Variables|/Game/Widgets/WBP_NearbyActions_Element.WBP_NearbyActions_Element_C|GetNearbyAction _aswbp_nearby_actions_element)))))
      (:Environment
        ;[1 1 1] Environment
        (Development|PrintString "Environment")))))

(event EventBeginPlay
  (bind _returnvalue (Components|GetOwner))
  (bind _returnvalue_2 (Components|GetOwner))
  (Utilities|FlowControl|Sequence
    (:then_0
      ;[1 1 1] Initialize widgets
      (bind _returnvalue_3 (UserInterface|CreateWidget "/Game/Widgets/WBP_NearbyActions.WBP_NearbyActions_C"))
      (Variables|Default|SetNearbyActionsWidget _returnvalue_3))
    (:then_1
      ;[1 1 1] Define InteractorActorComponent
      (if (Utilities|DoesObjectImplementInterface _returnvalue_2 "/Game/Prototype/ActorComponents/BPI_ActorComponentInteractor_Holder.BPI_ActorComponentInteractor_Holder_C")
        (bind _component (Class|BPIActorComponentInteractorHolder|GetInteractorActorComponent(Message) _returnvalue_2))
        (Variables|Default|SetInteractorActorComponent _component)
        (else
          (Development|PrintString "Error: Owner doesn't implements interface" true true "(R=1.000000,G=0.000000,B=0.093436,A=1.000000)"))))
    (:then_2
      ;[1 1 1] Define InventoryActorComponent
      (if (Utilities|DoesObjectImplementInterface _returnvalue "/Script/Sas3.InventoryActorComponentHolder")
        (bind _returnvalue_4 (Class|InventoryActorComponentHolder|GetInventoryActorComponent(Message) _returnvalue))
        (Variables|Default|SetInventoryActorComponent _returnvalue_4)
        (else
          (Development|PrintString "Error: Owner doesn't implements InventoryActorComponent interface" true true "(R=1.000000,G=0.000000,B=0.093436,A=1.000000)"))))))