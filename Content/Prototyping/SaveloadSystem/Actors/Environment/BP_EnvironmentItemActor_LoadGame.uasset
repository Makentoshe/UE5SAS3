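; Prototype environment actor for the save/load system that loads the current general save slot when interacted with.
; Its interactable sphere component triggers the load through the Saveload game instance subsystem.
; BeginPlay binds to that subsystem's async load started and completed events, which currently only print debug messages.
; The Cube mesh is exposed for outlining, and animation and VFX feedback remain a TODO.
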(event OnInteractionAction(BP_InteractableSphereComponent)
  (params (InteractedActor :type Actor%20Object%20Reference) (InteractionWrapper :type Interaction%20Wrapper%20Object%20Reference))
  ;[1 1 1] Chest opening
  ; TODO: Play animation and vfx effects
  (Class|SaveloadGameInstanceSubsystem|LoadCurrentGeneralSaveloadSlot (Subsystems|GetSaveloadGameInstanceSubsystem)))

(event Custom|OnAsyncLoadGameStarted_Event_0
  (params (Structure :type Saveload%20Slot%20Structure%20Structure))
  (Development|PrintString "Loading started"))

(event Custom|OnAsyncLoadGameCompleted_Event_0
  (params (LoadGameGeneral :type Save%20Game%20General%20Object%20Reference))
  (Development|PrintString "Loading completed"))

(event EventBeginPlay
  (EventDispatchers|AssignOnAsyncLoadGameStarted (Subsystems|GetSaveloadGameInstanceSubsystem) (delegate Custom|OnAsyncLoadGameStarted_Event_0))
  (EventDispatchers|AssignOnAsyncLoadGameCompleted (Subsystems|GetSaveloadGameInstanceSubsystem) (delegate Custom|OnAsyncLoadGameCompleted_Event_0)))

(fn ConstructionScript
  (|CallParentFunction))

(fn GetOutlinableMeshComponents
  (return (Utilities|Array|MakeArray (Variables|Default|GetCube))))