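; Prototype environment item actor that saves the game to the current general saveload slot when a player interacts with its sphere component.
; On BeginPlay it binds to the SaveloadGameInstanceSubsystem's delegates for save instance creation, actor serialization and async save start and completion, and unbinds on EndPlay.
; Each callback prints a debug string to trace the save process.
; Its Cube mesh is exposed as the outlinable component.
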(event OnInteractionAction(BP_InteractableSphereComponent)
  (params (InteractedActor :type Actor%20Object%20Reference) (InteractionWrapper :type Interaction%20Wrapper%20Object%20Reference))
  (Class|SaveloadGameInstanceSubsystem|SaveCurrentGeneralSaveloadSlot (Subsystems|GetSaveloadGameInstanceSubsystem)))

(event Custom|OnActorSerialized_Event_0
  (params (SerializedActor :type Actor%20Object%20Reference) (Structure :type Saveload%20Actor%20Structure%20Structure))
  (Development|PrintString (Utilities|GetDisplayName SerializedActor) true true "(R=0.504483,G=0.000000,B=1.000000,A=1.000000)"))

(event Custom|OnAsyncSaveGameStarted_Event_0
  (params (Structure :type Saveload%20Slot%20Structure%20Structure) (SaveGameGeneral :type Save%20Game%20General%20Object%20Reference))
  (Development|PrintString "Start savegame"))

(event Custom|OnAsyncSaveGameCompleted_Event_0
  (params (SlotName :type String) (UserIndex :type Integer) (bSuccess :type Boolean))
  (Development|PrintString "Savegame finished"))

(event Custom|OnGeneralSaveGameInstanceCreated_Event_0
  (params (SaveGameGeneral :type Save%20Game%20General%20Object%20Reference))
  (Development|PrintString (Utilities|GetDisplayName SaveGameGeneral)))

(event EventBeginPlay
  (bind _returnvalue (Subsystems|GetSaveloadGameInstanceSubsystem))
  (bind _returnvalue_2 (Subsystems|GetSaveloadGameInstanceSubsystem))
  (EventDispatchers|AssignOnGeneralSaveGameInstanceCreated _returnvalue (delegate Custom|OnGeneralSaveGameInstanceCreated_Event_0))
  (EventDispatchers|AssignOnActorSerialized _returnvalue (delegate Custom|OnActorSerialized_Event_0))
  (EventDispatchers|AssignOnAsyncSaveGameStarted _returnvalue_2 (delegate Custom|OnAsyncSaveGameStarted_Event_0))
  (EventDispatchers|AssignOnAsyncSaveGameCompleted _returnvalue_2 (delegate Custom|OnAsyncSaveGameCompleted_Event_0)))

(event EventEndPlay
  (params (EndPlayReason :type EEndPlayReason%20Enum :default "Destroyed"))
  (bind _returnvalue (Subsystems|GetSaveloadGameInstanceSubsystem))
  (bind _returnvalue_2 (Subsystems|GetSaveloadGameInstanceSubsystem))
  (EventDispatchers|UnbindEventfromOnGeneralSaveGameInstanceCreated _returnvalue (delegate Custom|OnGeneralSaveGameInstanceCreated_Event_0))
  (EventDispatchers|UnbindEventfromOnActorSerialized _returnvalue (delegate Custom|OnActorSerialized_Event_0))
  (EventDispatchers|UnbindEventfromOnAsyncSaveGameStarted _returnvalue_2 (delegate Custom|OnAsyncSaveGameStarted_Event_0))
  (EventDispatchers|UnbindEventfromOnAsyncSaveGameCompleted _returnvalue_2 (delegate Custom|OnAsyncSaveGameCompleted_Event_0)))

(fn ConstructionScript
  (|CallParentFunction))

(fn GetOutlinableMeshComponents
  (return (Utilities|Array|MakeArray (Variables|Default|GetCube))))