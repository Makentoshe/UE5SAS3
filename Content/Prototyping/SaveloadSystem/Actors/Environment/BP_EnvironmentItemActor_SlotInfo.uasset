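; BP_EnvironmentItemActor_SlotInfo is a prototype interactable environment actor that reports the current save slot for the save/load system.
; When its interactable sphere component fires an interaction, it reads the current general slot from the save/load game instance subsystem and prints the filename and initialized state.
; It exposes its Cube mesh as the outlinable component.
; A leftover TODO mentions chest-opening animation and VFX, which are not implemented.
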(event OnInteractionAction(BP_InteractableSphereComponent)
  (params (InteractedActor :type Actor%20Object%20Reference) (InteractionWrapper :type Interaction%20Wrapper%20Object%20Reference))
  ;[1 1 1] Chest opening
  ; TODO: Play animation and vfx effects
  (bind _returnvalue (Class|SaveloadGameInstanceSubsystem|GetCurrentGeneralSaveloadSlot (Subsystems|GetSaveloadGameInstanceSubsystem)))
  (Development|PrintString (Utilities|String|Append "SlotTitle=" (.Filename (Utilities|Struct|BreakSaveloadSlotStructure _returnvalue)) ", Initialized=" (Utilities|String|ToString(Boolean) (.IsInitialized (Utilities|Struct|BreakSaveloadSlotStructure _returnvalue))))))

(fn ConstructionScript
  (|CallParentFunction))

(fn GetOutlinableMeshComponents
  (return (Utilities|Array|MakeArray (Variables|Default|GetCube))))