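; Test pawn that shows an info display when its interaction component is selected.
; Selection passes a placeholder label and short description to the display widget component, while unselection or unavailability hides it.
; It exposes its interaction component through a getter and includes a helper that checks an actor for the InteractorComponentHolder interface and fetches its interactor component.
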(event OnInteractionComponentSelectedDelegate(BP_InteractionComponent)
  (Class|InfoDisplayWidgetComponent|ShowDisplayWidget (Variables|Default|GetBP_InfoDisplayWidgetComponent) (Utilities|Struct|MakeSDisplayInfo "Label String" "Short description string")))

(event OnInteractionComponentUnselectedDelegate(BP_InteractionComponent)
  (Class|DisplayWidgetComponent|HideDisplayWidget (Variables|Default|GetBP_InfoDisplayWidgetComponent)))

(event OnInteractionComponentUnavailableDelegate(BP_InteractionComponent)
  (Class|DisplayWidgetComponent|HideDisplayWidget (Variables|Default|GetBP_InfoDisplayWidgetComponent)))

(fn ConstructionScript)

(fn GetInteractionComponent
  (return (Variables|Default|GetBP_InteractionComponent)))