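; Actor component that manages the nearby-interaction UI for its owner and carries out the selected action.
; On BeginPlay it creates the interaction widgets and fetches the owner's interactor and inventory components through interfaces.
; Events forward entry and selection changes to the character interaction widget, showing or hiding it as entries change.
; Interacting branches on action type: inventory items are added and destroyed, environment items run their own event.
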(event Custom|OnAddNearbyActionEvent
  (params (NearbyActionWrapper :type A%20Nearby%20Action%20Structure%20Wrapper%20Object%20Reference))
  (bind _characterinteractionswidget (Variables|Default|GetCharacterInteractionsWidget))
  ;[1 1 1] Adding NearbyAction to the UI
  (Default|OnAddNearbyInteractionEntryEvent _characterinteractionswidget NearbyActionWrapper)
  (if (not (Widget|IsVisible _characterinteractionswidget))
    (UserInterface|Viewport|AddtoViewport _characterinteractionswidget 0)))

(event Custom|OnRemoveNearbyActionEvent
  (params (NearbyActionWrapper :type A%20Nearby%20Action%20Structure%20Wrapper%20Object%20Reference))
  (bind _characterinteractionswidget (Variables|Default|GetCharacterInteractionsWidget))
  ;[1 1 1] Removing NearbyAction from the UI
  (Default|OnRemoveNearbyInteractionEntryEvent _characterinteractionswidget NearbyActionWrapper)
  (if (not (> (Class|ListView|GetNumItems (Variables|/Game/Widgets/WBP_CharacterInteraction.WBP_CharacterInteraction_C|GetInteractionActionsContainer _characterinteractionswidget)) 0))
    (Widget|RemovefromParent _characterinteractionswidget)))

(event Custom|OnChangeSelectedNearbyActionIndexEvent
  (params (NewIndex :type Integer))
  ;[1 1 1] NearbyAction selection scrolling
  (Default|OnNearbyInteractionSelectionChangedEvent (Variables|Default|GetCharacterInteractionsWidget) NewIndex))

(event Custom|OnNearbyActionInteractionEvent
  (params (NearbyActionSelectedIndex :type Integer))
  ;[1 1 1] Get selected NearbyAction widget
  (if (Widget|IsVisible (Variables|Default|GetCharacterInteractionsWidget))
    (bind _asa_nearby_action_structure_wrapper (Utilities|Casting|CastToA_NearbyActionStructureWrapper (Class|ListView|GetItemat (Variables|/Game/Widgets/WBP_CharacterInteraction.WBP_CharacterInteraction_C|GetInteractionActionsContainer (Variables|Default|GetCharacterInteractionsWidget)) NearbyActionSelectedIndex))
      (:then
        ;[1 1 1] Get NearbyAction type
        (switch Utilities|FlowControl|Switch|SwitchonE_NearbyActionType (.ActionType (Utilities|Struct|BreakS_NearbyActionStructure (Variables|/Game/Structure/A_NearbyActionStructureWrapper.A_NearbyActionStructureWrapper_C|GetNearbyActionStructure _asa_nearby_action_structure_wrapper)))
          (:NewEnumerator0
            (Development|PrintString "Error: NearbyAction type is None" true true "(R=1.000000,G=0.010790,B=0.000000,A=1.000000)" :!pinned true) ; None: shouldn't be reachable
          )
          (:NewEnumerator1
            ;[1 1 1] Add item to the Inventory and destroy the actor
            (bind _asbp_inventory_item_actor (Utilities|Casting|CastToBP_InventoryItemActor (.GameItemActor (Utilities|Struct|BreakS_NearbyActionStructure (Variables|/Game/Structure/A_NearbyActionStructureWrapper.A_NearbyActionStructureWrapper_C|GetNearbyActionStructure _asa_nearby_action_structure_wrapper))))
              (:then
                (Class|InventoryActorComponent|AddInventoryItem (Variables|Default|GetInventoryActorComponent) (Utilities|Struct|MakeInventoryItemStructure (.ItemCount (Utilities|Struct|BreakS_InventoryMetaStructure (Variables|/Game/Actor/BP_InventoryItemActor.BP_InventoryItemActor_C|GetInventoryMeta _asbp_inventory_item_actor))) (.StackSize (Utilities|Struct|BreakS_InventoryMetaStructure (Variables|/Game/Actor/BP_InventoryItemActor.BP_InventoryItemActor_C|GetInventoryMeta _asbp_inventory_item_actor))) (Utilities|Struct|BreakS_GameItemStructure (Variables|/Game/Actor/BP_GameItemActor.BP_GameItemActor_C|GetGameItem _asbp_inventory_item_actor))))
                (Actor|DestroyActor (.GameItemActor (Utilities|Struct|BreakS_NearbyActionStructure (Variables|/Game/Structure/A_NearbyActionStructureWrapper.A_NearbyActionStructureWrapper_C|GetNearbyActionStructure _asa_nearby_action_structure_wrapper)))))
              (:CastFailed
                (Development|PrintString "Error: Cant cast object to InventoryItemActor" true true "(R=1.000000,G=0.938499,B=0.000000,A=1.000000)"))))
          (:NewEnumerator2
            ;[1 1 1] Execute Environment action
            (bind _asbp_environment_item_actor (Utilities|Casting|CastToBP_EnvironmentItemActor (.GameItemActor (Utilities|Struct|BreakS_NearbyActionStructure (Variables|/Game/Structure/A_NearbyActionStructureWrapper.A_NearbyActionStructureWrapper_C|GetNearbyActionStructure _asa_nearby_action_structure_wrapper))))
              (:then
                (Default|OnEnvironmentNearbyActionEvent _asbp_environment_item_actor))
              (:CastFailed
                (Development|PrintString "Error: Cant cast object to EnvironmentItemActor" true true "(R=1.000000,G=0.938499,B=0.000000,A=1.000000)"))))))
      (:CastFailed
        (Development|PrintString "Error: Cant cast item to NearbyActionStructureWrapper" true true "(R=1.000000,G=0.000000,B=0.030146,A=1.000000)")))
    (else
      (Development|PrintString "Error: NearbyInteractionsWidget isn't visible - cant interact with the items" true true "(R=1.000000,G=0.000000,B=0.026892,A=1.000000)"))))

(event Custom|OnNearbyInteractionSelectionChangedEvent
  (params (NewSelectionIndex :type Integer))
  ;[1 1 1] Nearby selection changed via setter
  (Default|OnNearbyInteractionSelectionChangedEvent (Variables|Default|GetCharacterInteractionsWidget) NewSelectionIndex))

(event EventBeginPlay
  (bind _returnvalue (Components|GetOwner))
  (bind _returnvalue_2 (Components|GetOwner))
  (Utilities|FlowControl|Sequence
    (:then_0
      ;[1 1 1] Initialize widgets
      (bind _returnvalue_3 (UserInterface|CreateWidget "/Game/Widgets/WBP_NearbyActions.WBP_NearbyActions_C"))
      (Variables|Default|SetNearbyActionsWidget _returnvalue_3)
      (bind _returnvalue_4 (UserInterface|CreateWidget "/Game/Widgets/WBP_CharacterInteraction.WBP_CharacterInteraction_C"))
      (Variables|Default|SetCharacterInteractionsWidget _returnvalue_4))
    (:then_1
      ;[1 1 1] Define InteractorActorComponent
      (if (Utilities|DoesObjectImplementInterface _returnvalue_2 "/Game/Interface/BPI_ActorComponentInteractor_Holder.BPI_ActorComponentInteractor_Holder_C")
        (bind _component (Class|BPIActorComponentInteractorHolder|GetInteractorActorComponent(Message) _returnvalue_2))
        (Variables|Default|SetInteractorActorComponent _component)
        (else
          (Development|PrintString "Error: Owner doesn't implements interface" true true "(R=1.000000,G=0.000000,B=0.093436,A=1.000000)"))))
    (:then_2
      ;[1 1 1] Define InventoryActorComponent
      (if (Utilities|DoesObjectImplementInterface _returnvalue "/Script/Sas3.InventoryActorComponentHolder")
        (bind _returnvalue_5 (Class|InventoryActorComponentHolder|GetInventoryActorComponent(Message) _returnvalue))
        (Variables|Default|SetInventoryActorComponent _returnvalue_5)
        (else
          (Development|PrintString "Error: Owner doesn't implements InventoryActorComponent interface" true true "(R=1.000000,G=0.000000,B=0.093436,A=1.000000)"))))))