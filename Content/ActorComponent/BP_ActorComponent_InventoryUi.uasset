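; Actor component that shows and hides the character inventory UI for the third-person player.
; On BeginPlay it caches the owner's inventory component through the InventoryActorComponentHolder interface, plus the owning character and its player controller.
; The show event creates the inventory widget, fills it from that component, and switches to Game-and-UI input with a mouse cursor.
; The hide event discards the widget and restores game-only input.
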(event Custom|OnShowInventoryWidgetEvent
  ;[1 1 1] Create inventory widget
  (bind _returnvalue (UserInterface|CreateWidget "/Game/Widgets/WBP_CharacterInventory.WBP_CharacterInventory_C" (Variables|Owner|GetThirdPersonPlayerController)))
  (bind _output_get (Variables|UserInterface|SetInventoryWidget _returnvalue))
  ;[1 1 1] Fill inventory widget with items
  (Default|UpdateInventoryEntries _output_get (Variables|Default|GetInventoryActorComponent))
  ;[1 1 1] Get controll from the player
  (Input|SetInputModeGameandUI (Variables|Owner|GetThirdPersonPlayerController) (Variables|UserInterface|GetInventoryWidget) "DoNotLock" true)
  (UserInterface|Viewport|AddtoViewport (Variables|UserInterface|GetInventoryWidget) 0)
  (Variables|/Script/Engine.PlayerController|SetbShowMouseCursor (Variables|Owner|GetThirdPersonPlayerController) true))

(event Custom|OnHideInventoryWidgetEvent
  (bind _thirdpersonplayercontroller (Variables|Owner|GetThirdPersonPlayerController))
  ;[1 1 1] Remove inventory widget
  (Widget|RemovefromParent (Variables|UserInterface|GetInventoryWidget))
  (Variables|UserInterface|SetInventoryWidget 0)
  ;[1 1 1] Return controll to the player
  (Input|SetInputModeGameOnly _thirdpersonplayercontroller)
  (Variables|/Script/Engine.PlayerController|SetbShowMouseCursor _thirdpersonplayercontroller false))

(event EventBeginPlay
  (bind _returnvalue (Components|GetOwner))
  (Utilities|FlowControl|Sequence
    (:then_0
      ;[1 1 1] Define InventoryActorComponent
      (if (Utilities|DoesObjectImplementInterface _returnvalue "/Script/Sas3.InventoryActorComponentHolder")
        (bind _returnvalue_2 (Class|InventoryActorComponentHolder|GetInventoryActorComponent(Message) _returnvalue))
        (Variables|Default|SetInventoryActorComponent _returnvalue_2)
        (else
          (Development|PrintString "Error: Owner doesn't implements InventoryActorComponentHolder interface" true true "(R=1.000000,G=0.000000,B=0.093436,A=1.000000)"))))
    (:then_1
      ;[1 1 1] Define ThirdPersonCharacter and ThirdPersonPlayerController
      (bind _asbp_third_person_character (Utilities|Casting|CastToBP_ThirdPersonCharacter (Components|GetOwner))
        (:then
          (bind _output_get (Variables|Owner|SetThirdPersonCharacter _asbp_third_person_character))
          (bind _asthird_person_player_controller (Utilities|Casting|CastToThirdPersonPlayerController (Pawn|GetController _output_get))
            (:then
              (Variables|Owner|SetThirdPersonPlayerController _asthird_person_player_controller))
            (:CastFailed
              (Development|PrintString "Error: Component wasn't attached to ThirdPersonPlayerController" true true "(R=1.000000,G=0.000000,B=0.179738,A=1.000000)"))))
        (:CastFailed
          (Development|PrintString "Error: Component wasn't attached to ThordpersonCharacter" true true "(R=1.000000,G=0.000000,B=0.179738,A=1.000000)"))))))