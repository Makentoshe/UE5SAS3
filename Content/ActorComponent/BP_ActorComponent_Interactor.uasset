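; Interactor component that tracks nearby actions and lets the owner cycle through and trigger the selected one.
; Each action is wrapped in a spawned A_NearbyActionStructureWrapper, stored in a map and parallel array; removal clears only the map entry.
; Changes go to the owner's InteractorUi component, fetched by interface like the inventory component.
; Interacting dispatches by action type: inventory items are added and destroyed, environment items receive an action event.
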(event Custom|OnAddNearbyActionEvent
  (params (NearbyActionStructure :type S%20Nearby%20Action%20Structure%20Structure))
  ;[1 1 1] Add NearbyInteraction structure to the map
  (bind _wrapped (Utilities|Wrap NearbyActionStructure)
    (:%20%20
      (Utilities|Map|Add (Variables|Default|GetNearbyInteractions) NearbyActionStructure _wrapped)
      (Utilities|Array|Add (Variables|Default|GetNearbyInteractionWrappers) _wrapped)
      (Default|OnAddNearbyActionEvent (Variables|Default|GetInteractorUiActorComponent) _wrapped))))

(event Custom|OnRemoveNearbyActionEvent
  (params (NearbyActionStructure :type S%20Nearby%20Action%20Structure%20Structure))
  ;[1 1 1] Remove NearbyInteractionStructure from the map
  (bind _wrapper (CallFunction|FindWrapper (Variables|Default|GetNearbyInteractionWrappers) NearbyActionStructure))
  (if (.ReturnValue (Utilities|Map|Find (Variables|Default|GetNearbyInteractions) NearbyActionStructure)) ; Is map contains the item
    (Default|OnRemoveNearbyActionEvent (Variables|Default|GetInteractorUiActorComponent) _wrapper)
    (bind _returnvalue (Utilities|Map|Remove (Variables|Default|GetNearbyInteractions) NearbyActionStructure))
    (if _returnvalue ; If item was removed
      (bind _output_get (Variables|Default|SetSelectedNearbyInteractionIndex (Math|Integer|Max(Integer) (Math|Integer|Min(Integer) (- (Utilities|Map|Length (Variables|Default|GetNearbyInteractions)) 1) (Variables|Default|GetSelectedNearbyInteractionIndex)))))
      (Default|OnChangeSelectedNearbyActionIndexEvent (Variables|Default|GetInteractorUiActorComponent) _output_get)
      (Development|PrintString (Utilities|String|Append (Utilities|String|ToString(Integer) _output_get) " - " (Utilities|GetDisplayName (.GameItemActor (Utilities|Struct|BreakS_NearbyActionStructure NearbyActionStructure)))))
      (else
        (Development|PrintString "Error: Cant remove NearbyInteractionsWrapper from the map" true true "(R=1.000000,G=0.000000,B=0.070807,A=1.000000)")))
    (else
      (Development|PrintString "Error: Cant find NearbyInteractionsWrapper in the map" true true "(R=1.000000,G=0.000000,B=0.070807,A=1.000000)"))))

(event Custom|OnPrevSelectedNearbyInteractionIndexEvent
  ;[1 1 1] On Previous item selection event
  (if (< (- (Variables|Default|GetSelectedNearbyInteractionIndex) 1) 0)
    (Variables|Default|SetSelectedNearbyInteractionIndex (Math|Integer|Max(Integer) (- (Utilities|Array|Length (Variables|Default|GetNearbyInteractionWrappers)) 1)))
    (else
      (Variables|Default|SetSelectedNearbyInteractionIndex (- (Variables|Default|GetSelectedNearbyInteractionIndex) 1))))
  (Default|OnChangeSelectedNearbyActionIndexEvent (Variables|Default|GetInteractorUiActorComponent) (Variables|Default|GetSelectedNearbyInteractionIndex)))

(event Custom|OnNextSelectedNearbyInteractionIndexEvent
  ;[1 1 1] On Next item selection event
  (if (< (+ (Variables|Default|GetSelectedNearbyInteractionIndex) 1) (Utilities|Array|Length (Variables|Default|GetNearbyInteractionWrappers)))
    (Variables|Default|SetSelectedNearbyInteractionIndex (+ (Variables|Default|GetSelectedNearbyInteractionIndex) 1))
    (else
      (Variables|Default|SetSelectedNearbyInteractionIndex 0)))
  (Default|OnChangeSelectedNearbyActionIndexEvent (Variables|Default|GetInteractorUiActorComponent) (Variables|Default|GetSelectedNearbyInteractionIndex)))

(event Custom|OnNearbyInteractionEvent
  ;[1 1 1] Player somehow interacts with this item
  (if (!= (Utilities|Array|Length (Variables|Default|GetNearbyInteractionWrappers)) 0) ; If not empty interactions
    (if (> (Utilities|Array|Length (Variables|Default|GetNearbyInteractionWrappers)) (Variables|Default|GetSelectedNearbyInteractionIndex)) ; If selection value valid
      (bind _values (Utilities|Map|Values (Variables|Default|GetNearbyInteractions)))
      (CallFunction|InternalonNearbyInteraction (Utilities|Array|Get(acopy) (Variables|Default|GetNearbyInteractionWrappers) (Variables|Default|GetSelectedNearbyInteractionIndex)))
      (else
        (Development|PrintString "Error: Issue with NearbyInteractions list and selection" true true "(R=1.000000,G=0.000000,B=0.026892,A=1.000000)")))
    (else
      (Development|PrintString "Error: NearbyInteractionsWidget isn't visible - cant interact with the items" true true "(R=1.000000,G=0.000000,B=0.026892,A=1.000000)"))))

(event EventEndPlay
  (params (EndPlayReason :type EEndPlayReason%20Enum :default "Destroyed"))
  ;[1 1 1] Releasse
  (Utilities|Map|Clear (Variables|Default|GetNearbyInteractions))
  (Variables|Default|SetInteractorUiActorComponent 0)
  (Variables|Default|SetInventoryActorComponent 0)
  (Utilities|Array|Clear (Variables|Default|GetNearbyInteractionWrappers)))

(event EventBeginPlay
  (bind _returnvalue (Components|GetOwner))
  (bind _returnvalue_2 (Components|GetOwner))
  ;[1 1 1] replace to OnInitializeComponent
  (Utilities|FlowControl|Sequence
    (:then_0
      ;[1 1 1] Define InteractorUiActorComponent
      (if (Utilities|DoesObjectImplementInterface _returnvalue_2 "/Game/Interface/BPI_ActorComponent_InteractorUi_Holder.BPI_ActorComponent_InteractorUi_Holder_C")
        (bind _interactoruicomponent (Class|BPIActorComponentInteractorUiHolder|GetInteractorUiActorComponent(Message) _returnvalue_2))
        (Variables|Default|SetInteractorUiActorComponent _interactoruicomponent)
        (else
          (Development|PrintString "Error: Owner doesn't implements   interface" true true "(R=1.000000,G=0.000000,B=0.093436,A=1.000000)"))))
    (:then_1
      ;[1 1 1] Define InventoryActorComponent
      (if (Utilities|DoesObjectImplementInterface _returnvalue "/Script/Sas3.InventoryActorComponentHolder")
        (bind _returnvalue_3 (Class|InventoryActorComponentHolder|GetInventoryActorComponent(Message) _returnvalue))
        (Variables|Default|SetInventoryActorComponent _returnvalue_3)
        (else
          (Development|PrintString "Error: Owner doesn't implements InventoryActorComponent interface" true true "(R=1.000000,G=0.000000,B=0.093436,A=1.000000)"))))))

(event Input|KeyboardEvents|Tab
  (params (Key :type Key%20Structure :default "None"))
  (:Pressed
    (bind _values (Utilities|Map|Values (Variables|Default|GetNearbyInteractions)))
    (for (_array_element _array_index) _values
      (bind _asa_nearby_action_structure_wrapper (Utilities|Casting|CastToA_NearbyActionStructureWrapper _array_element))
      (Development|PrintString (Utilities|String|Append (Utilities|String|ToString(Integer) _array_index) " - " (Utilities|GetDisplayName (.GameItemActor (Utilities|Struct|BreakS_NearbyActionStructure (Variables|/Game/Structure/A_NearbyActionStructureWrapper.A_NearbyActionStructureWrapper_C|GetNearbyActionStructure _asa_nearby_action_structure_wrapper)))))))
    (Development|PrintString (Utilities|String|ToString(Integer) (Variables|Default|GetSelectedNearbyInteractionIndex)) true true "(R=1.000000,G=0.964452,B=0.000000,A=1.000000)")))

(fn InternalonNearbyInteraction
  (params (NearbyInteractionWrapper :type A%20Nearby%20Action%20Structure%20Wrapper%20Object%20Reference))
  (bind _nearbyactionstructure (Variables|/Game/Structure/A_NearbyActionStructureWrapper.A_NearbyActionStructureWrapper_C|GetNearbyActionStructure NearbyInteractionWrapper))
  (bind (_title _description _actiontype _gameitemactor) (Utilities|Struct|BreakS_NearbyActionStructure _nearbyactionstructure))
  (LocalVariables|SetNearbyInteractionStructure _nearbyactionstructure)
  (switch Utilities|FlowControl|Switch|SwitchonE_NearbyActionType _actiontype
    (:NewEnumerator0
      (Development|PrintString "Error: NearbyAction type is None" true true "(R=1.000000,G=0.010790,B=0.000000,A=1.000000)" :!pinned true) ; None: shouldn't be reachable
    )
    (:NewEnumerator1
      ;[1 1 1] Inventory interaction
      (bind _asbp_inventory_item_actor (Utilities|Casting|CastToBP_InventoryItemActor _gameitemactor)
        (:then
          (CallFunction|InternalonInventoryInteraction _asbp_inventory_item_actor))
        (:CastFailed
          (Development|PrintString "Error: Cant cast object to InventoryItemActor" true true "(R=1.000000,G=0.938499,B=0.000000,A=1.000000)"))))
    (:NewEnumerator2
      ;[1 1 1] Environment interaction
      (bind _asbp_environment_item_actor (Utilities|Casting|CastToBP_EnvironmentItemActor _gameitemactor)
        (:then
          (CallFunction|InternalonEnvironmentInteraction _asbp_environment_item_actor))
        (:CastFailed
          (Development|PrintString "Error: Cant cast object toEnvironmentItemActor" true true "(R=1.000000,G=0.938499,B=0.000000,A=1.000000)"))))))

(fn InternalonInventoryInteraction
  (params (InventoryItemActor :type BP%20Inventory%20Item%20Actor%20Object%20Reference))
  (bind _inventorymeta (Variables|/Game/Actor/BP_InventoryItemActor.BP_InventoryItemActor_C|GetInventoryMeta InventoryItemActor))
  (bind (_itemcount _stacksize) (Utilities|Struct|BreakS_InventoryMetaStructure _inventorymeta))
  (Utilities|FlowControl|Sequence
    (:then_0
      ;[1 1 1] Add item to the inventory
      (Class|InventoryActorComponent|AddInventoryItem (Variables|Default|GetInventoryActorComponent) (Utilities|Struct|MakeInventoryItemStructure _itemcount _stacksize (Utilities|Struct|BreakS_GameItemStructure (Variables|/Game/Actor/BP_GameItemActor.BP_GameItemActor_C|GetGameItem InventoryItemActor)))))
    (:then_1
      (Actor|DestroyActor InventoryItemActor :!pinned true) ; Destroying will cause OnEndOverlap which cause widget update
    )
    (:then_2
      ;[1 1 1] Decrease index if it out of the length bound
      (bind _output_get (Variables|Default|SetSelectedNearbyInteractionIndex (Math|Integer|Max(Integer) (Math|Integer|Min(Integer) (- (Utilities|Map|Length (Variables|Default|GetNearbyInteractions)) 1) (Variables|Default|GetSelectedNearbyInteractionIndex)))))
      (Default|OnChangeSelectedNearbyActionIndexEvent (Variables|Default|GetInteractorUiActorComponent) _output_get))))

(fn InternalonEnvironmentInteraction
  (params (EnvironmentItemActor :type BP%20Environment%20Item%20Actor%20Object%20Reference))
  (Default|OnEnvironmentNearbyActionEvent EnvironmentItemActor))

(fn FindWrapper
  (params (Array :type Array%20of%20A%20Nearby%20Action%20Structure%20Wrapper%20Object%20References) (NearbyActionStructure :type S%20Nearby%20Action%20Structure%20Structure))
  (for _array_element Array
    (bind __ (CallFunction|Equals (Variables|/Game/Structure/A_NearbyActionStructureWrapper.A_NearbyActionStructureWrapper_C|GetNearbyActionStructure _array_element) NearbyActionStructure))
    (if __
      (return _array_element __)))
  (return 0 false))