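; BP_EnvironmentItemActor is an environment game item that offers a nearby action to actors entering its interaction sphere.
; Sphere overlaps check for the interactor-holder interface, then add or remove a nearby action on that actor's interactor component.
; The action structure carries the item title, environment description and a self reference.
; OnEnvironmentNearbyActionEvent is an empty stub, and construction defers to the parent.
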(event OnComponentBeginOverlap(InteractionSphereComponent)
  (params (OverlappedComponent :type Primitive%20Component%20Object%20Reference) (OtherActor :type Actor%20Object%20Reference) (OtherComp :type Primitive%20Component%20Object%20Reference) (OtherBodyIndex :type Integer) (bFromSweep :type Boolean) (SweepResult :type Hit%20Result%20Structure%20%28by%20ref%29))
  (if (Utilities|DoesObjectImplementInterface OtherActor "/Game/Interface/BPI_ActorComponentInteractor_Holder.BPI_ActorComponentInteractor_Holder_C")
    (bind _component (Class|BPIActorComponentInteractorHolder|GetInteractorActorComponent(Message) OtherActor))
    (Default|OnAddNearbyActionEvent _component (Utilities|Struct|MakeS_NearbyActionStructure (Utilities|Struct|BreakGameItemStructure (Variables|Default|GetGameItem)) (Utilities|Struct|BreakS_EnvironmentMetaStructure (Variables|Item|GetEnvironmentMeta)) "NewEnumerator2" self))))

(event OnComponentEndOverlap(InteractionSphereComponent)
  (params (OverlappedComponent :type Primitive%20Component%20Object%20Reference) (OtherActor :type Actor%20Object%20Reference) (OtherComp :type Primitive%20Component%20Object%20Reference) (OtherBodyIndex :type Integer))
  (if (Utilities|DoesObjectImplementInterface OtherActor "/Game/Interface/BPI_ActorComponentInteractor_Holder.BPI_ActorComponentInteractor_Holder_C")
    (bind _component (Class|BPIActorComponentInteractorHolder|GetInteractorActorComponent(Message) OtherActor))
    (Default|OnRemoveNearbyActionEvent _component (Utilities|Struct|MakeS_NearbyActionStructure (Utilities|Struct|BreakGameItemStructure (Variables|Default|GetGameItem)) (Utilities|Struct|BreakS_EnvironmentMetaStructure (Variables|Item|GetEnvironmentMeta)) "NewEnumerator2" self))))

(event Custom|OnEnvironmentNearbyActionEvent)

(fn ConstructionScript
  (|CallParentFunction))