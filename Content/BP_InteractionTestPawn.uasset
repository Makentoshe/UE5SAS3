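; BP_InteractionTestPawn is a test actor for the interaction system, carrying an interaction component and a text render.
; When an overlapping actor implements BPI_InteractorComponentHolder, it adds its interaction component to that actor's interactor component, removing it on end overlap.
; BeginPlay binds the component's enabled, disabled and removed events to show or hide the text.
; Getter functions expose the interaction component.
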(event OnComponentBeginOverlap(BP_InteractionComponent)
  (params (OverlappedComponent :type Primitive%20Component%20Object%20Reference) (OtherActor :type Actor%20Object%20Reference) (OtherComp :type Primitive%20Component%20Object%20Reference) (OtherBodyIndex :type Integer) (bFromSweep :type Boolean) (SweepResult :type Hit%20Result%20Structure%20%28by%20ref%29))
  (bind _component (Utilities|DoesImplementInteractorComponentHolder OtherActor)
    (:True
      (Class|BPIInteractorComponent|AddInteractionComponent2(Message) _component (Variables|Default|GetBP_InteractionComponent)))))

(event OnComponentEndOverlap(BP_InteractionComponent)
  (params (OverlappedComponent :type Primitive%20Component%20Object%20Reference) (OtherActor :type Actor%20Object%20Reference) (OtherComp :type Primitive%20Component%20Object%20Reference) (OtherBodyIndex :type Integer))
  (bind _component (Utilities|DoesImplementInteractorComponentHolder OtherActor)
    (:True
      (Class|BPIInteractorComponent|RemoveInteractionComponent2(Message) _component (Variables|Default|GetBP_InteractionComponent)))))

(event Custom|OnComponentEnabled_Event
  (Rendering|SetVisibility (Variables|Default|GetTextRender) true false))

(event Custom|OnComponentDisabled_Event
  (Rendering|SetVisibility (Variables|Default|GetTextRender) false false))

(event EventBeginPlay
  (bind _bp_interactioncomponent (Variables|Default|GetBP_InteractionComponent))
  (EventDispatchers|AssignOnComponentEnabled (Variables|Default|GetBP_InteractionComponent) (delegate Custom|OnComponentEnabled_Event))
  (EventDispatchers|AssignOnComponentDisabled _bp_interactioncomponent (delegate Custom|OnComponentDisabled_Event))
  (EventDispatchers|AssignOnComponentRemoved _bp_interactioncomponent (delegate Custom|OnComponentDisabled_Event)))

(fn ConstructionScript)

(fn GetInteractionComponent
  (return (Variables|Default|GetBP_InteractionComponent)))

(fn GetInteractionComponent2
  (return (Variables|Default|GetBP_InteractionComponent)))