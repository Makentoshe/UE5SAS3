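; BP_ActorSupport is a set of helper functions for relative rotation, direction and placement of actors.
; CalculateRotationBetweenActors smoothly interpolates the source's rotation toward a yaw-only look-at of the target, using world delta time and a fixed speed.
; CalculateVectorDirection returns the unnormalized vector pointing from target to source.
; GetActorFrontTransform offsets an actor's transform along its forward vector by a given distance, keeping rotation and scale.
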(fn CalculateRotationBetweenActors
  (params (From%20%28Source%29 :type Actor%20Object%20Reference) (To%20%28Target%29 :type Actor%20Object%20Reference))
  (return (Math|Interpolation|RInterpTo (Transformation|GetActorRotation From%20%28Source%29) (Math|Rotator|MakeRotator 0.0 0.0 (.Yaw (Math|Rotator|BreakRotator (Math|Rotator|FindLookatRotation (Transformation|GetActorLocation From%20%28Source%29) (Transformation|GetActorLocation To%20%28Target%29))))) (Utilities|Time|GetWorldDeltaSeconds) 3.0)))

(fn CalculateVectorDirection
  (params (Source%20%28From%29 :type Actor%20Object%20Reference) (Target%20%28To%29 :type Actor%20Object%20Reference))
  (return (- (Transformation|GetActorLocation Source%20%28From%29) (Transformation|GetActorLocation Target%20%28To%29))))

(fn GetActorFrontTransform
  (params (Target :type Actor%20Object%20Reference) (Distance :type Float%20%28double-precision%29))
  (bind _returnvalue (Transformation|GetActorTransform Target))
  (bind (_location _rotation _scale) (Math|Transform|BreakTransform _returnvalue))
  (return (Math|Transform|MakeTransform (+ (* (Transformation|GetActorForwardVector Target) Distance) _location) _rotation _scale)))