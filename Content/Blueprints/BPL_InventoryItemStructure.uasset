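; Blueprint function library of helpers for the inventory item structure.
; ToDebugString formats an item's title, count and stack size into a readable string.
; ToActionStructure converts an item and its actor into a nearby-action structure, using the title as title, the count as description and a fixed action type.
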(fn ToDebugString
  (params (Item :type Inventory%20Item%20Structure%20Structure))
  (bind (_count _stacksize _title) (Utilities|Struct|BreakInventoryItemStructure Item))
  (return (Utilities|String|Append "InventoryItem(title=" (Utilities|String|ToString(Name) _title) ", Count=" (Utilities|String|ToString(Integer) _count) ", StackSize=" (Utilities|String|ToString(Integer) _stacksize) ")")))

(fn ToActionStructure
  (params (InventoryItem :type Inventory%20Item%20Structure%20Structure) (InventoryItemActor :type Game%20Item%20Actor%20Object%20Reference))
  (bind (_count _stacksize _title) (Utilities|Struct|BreakInventoryItemStructure InventoryItem))
  (return (Utilities|Struct|MakeS_NearbyActionStructure _title (Utilities|String|StringToName (Utilities|String|ToString(Integer) _count)) "NewEnumerator1" InventoryItemActor)))