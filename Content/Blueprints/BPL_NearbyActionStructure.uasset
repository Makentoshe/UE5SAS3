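; Blueprint function library of helper checks for the NearbyAction structure, which describes an action tied to a game item actor.
; Equals treats two actions as the same only when title, description, action type and game item actor all match.
; IsInitialized reports whether an action is filled in by testing that its title, action type and actor differ from their empty defaults, ignoring the description.
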(fn Equals
  (params (First :type S%20Nearby%20Action%20Structure%20Structure) (Second :type S%20Nearby%20Action%20Structure%20Structure))
  (bind (_title _description _actiontype _gameitemactor) (Utilities|Struct|BreakS_NearbyActionStructure First))
  (bind (_title_2 _description_2 _actiontype_2 _gameitemactor_2) (Utilities|Struct|BreakS_NearbyActionStructure Second))
  (return (Math|Boolean|ANDBoolean (== _title _title_2) (== _description _description_2) (Utilities|Enum|Equal(Enum) _actiontype _actiontype_2) (== _gameitemactor _gameitemactor_2))))

(fn IsInitialized
  (params (NearbyAction :type S%20Nearby%20Action%20Structure%20Structure))
  (bind (_title _description _actiontype _gameitemactor) (Utilities|Struct|BreakS_NearbyActionStructure NearbyAction))
  (return (Math|Boolean|ANDBoolean (!= _title "") (Utilities|Enum|NotEqual(Enum) _actiontype "NewEnumerator0") (!= _gameitemactor 0))))