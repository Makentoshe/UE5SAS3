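; Function library of helpers for the NearbyInteraction structure used to describe interactions.
; Equals compares two structures by title, description, interaction type and actor.
; IsInitialized tests the title, interaction type and actor against default values, expecting a set title but a None type.
; Wrap constructs a NearbyInteractionWrapper object under a given owner and stores the structure in it, so the struct can be handled as an object.
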(fn Equals
  (params (First :type Nearby%20Interaction%20Structure%20Structure) (Second :type Nearby%20Interaction%20Structure%20Structure))
  (bind (_title _description _nearbyinteractiontype _actor) (Utilities|Struct|BreakNearbyInteractionStructure First))
  (bind (_title_2 _description_2 _nearbyinteractiontype_2 _actor_2) (Utilities|Struct|BreakNearbyInteractionStructure Second))
  (return (Math|Boolean|ANDBoolean (== _title _title_2) (== _description _description_2) (Utilities|Enum|Equal(Enum) _nearbyinteractiontype _nearbyinteractiontype_2) (== _actor _actor_2))))

(fn IsInitialized
  (params (NearbyInteraction :type Nearby%20Interaction%20Structure%20Structure))
  (bind (_title _description _nearbyinteractiontype _actor) (Utilities|Struct|BreakNearbyInteractionStructure NearbyInteraction))
  (return (Math|Boolean|ANDBoolean (!= _title "") (Utilities|Enum|Equal(Enum) _nearbyinteractiontype "None") (== _actor 0))))

(fn Wrap
  (params (Structure :type Nearby%20Interaction%20Structure%20Structure) (Owner :type Object%20Object%20Reference))
  (bind _returnvalue (Game|ConstructObjectfromClass Owner "/Script/Sas3.NearbyInteractionWrapper"))
  (Variables|/Script/Sas3.NearbyInteractionWrapper|SetNearbyInteractionStructure _returnvalue Structure)
  (return _returnvalue))