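; Test pawn that shows a display label while its interaction component is selected.
; The selected delegate shows a label widget with placeholder text through the display component, and the unselected and unavailable delegates both hide it.
; It exposes its interaction component through a getter and includes a helper that checks whether an actor implements InteractorComponentHolder and, if so, fetches its interactor component.
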(event OnInteractionComponentSelectedDelegate(BP_InteractionComponent)
  (Class|LabelDisplayWidgetComponent|ShowDisplayWidget (Variables|Default|GetBP_DisplayComponent) (Utilities|Struct|MakeSDisplayLabel "Label Text")))

(event OnInteractionComponentUnselectedDelegate(BP_InteractionComponent)
  (Class|DisplayWidgetComponent|HideDisplayWidget (Variables|Default|GetBP_DisplayComponent)))

(event OnInteractionComponentUnavailableDelegate(BP_InteractionComponent)
  (Class|DisplayWidgetComponent|HideDisplayWidget (Variables|Default|GetBP_DisplayComponent)))

(fn ConstructionScript)

(fn GetInteractionComponent
  (return (Variables|Default|GetBP_InteractionComponent)))